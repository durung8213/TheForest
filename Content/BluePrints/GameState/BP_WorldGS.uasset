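; BP_WorldGS is a world GameState Blueprint that keeps a looping day clock.
; Tick adds delta seconds to CurrentTime and resets it to zero once it reaches DayLength.
; It then derives NormalizedTime as the fraction of the day elapsed, intended for smooth sun movement.
; The clock runs on accumulated frame time, as the GetServerWorldTimeSeconds node is left unused.
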(event `self.ReceiveTick`
  (params (DeltaSeconds :type "Float (single-precision)"))
  ;[1 1 1] Tick 으로 시간의 흐름을 구현.
  (set `self.CurrentTime` (+ DeltaSeconds (`self.CurrentTime`))) ; Tick 마다의 시간을 Time에 증가시키고
  (if (>= (`self.CurrentTime`) (`self.DayLength`))
    (set `self.CurrentTime` 0.0) ; 다시 초기화한다
  )
  (set `self.NormalizedTime` (/ (`self.CurrentTime`) (`self.DayLength`))) ; 노말라이즈 타임을 정해서 해가 자연스럽게 움직이도록 한다.
)

(fn `UserConstructionScript`
  (`parent.UserConstructionScript`))