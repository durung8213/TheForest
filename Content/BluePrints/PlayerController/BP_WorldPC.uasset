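; BP_WorldPC is the player controller for a multiplayer survival game, routing input to the character and WorldHUD and passing the player name to the server.
; A looping camera line trace flags items for pickup or buildings for interaction, driving the E key alongside craft mode.
; Building placement uses a timer-driven ghost preview with overlap validation.
; Server events delegate item destruction and ghost-craft spawning to game-mode managers, and light campfires.
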(event `OwnerGetName`
  ;[1 1 1] 플레이어 이름 설정
  (`/Engine/EditorBlueprintResources/ActorMacros.Switch Has Authority`
    (:`Remote`
      (bind _asbp_multi_forest_gi (cast `/Game/BluePrints/BP_MultiForestGI` (`GameplayStatics.GetGameInstance`)))
      (bind _playername (`/Game/BluePrints/BP_MultiForestGI.GetPlayerName` _asbp_multi_forest_gi))
      (bind _output_get (set `self.Player Name` _playername))
      (`self.ServerSetPlayerName` _output_get))))

(event `self.ReceiveBeginPlay`
  ;[1 1 1] 클라이언트 플레이어 : Line Trace
  (`self.OwnerGetName`)
  (`self.SetTimerForLineTrace`))

(event `InputAxis|MoveForward`
  (params (AxisValue :type "Float (single-precision)"))
  ;[1 1 1] 전후좌우 이동
  (bind _asbp_player_character (cast `/Game/Character/BP_PlayerCharacter` (`self.K2_GetPawn`)))
  (`Pawn.AddMovementInput` _asbp_player_character (`self.GetDirectionVector`) AxisValue false))

(event `InputAction|Dash`
  (params (Key :type "Key Structure"))
  ;[1 1 1] 대쉬
  (:`Pressed`
    (bind _asbp_player_character (cast `/Game/Character/BP_PlayerCharacter` (`self.K2_GetPawn`)))
    (`/Game/BluePrints/Class/BP_PlayerStatus.Owner_StartDash` (`/Game/Character/BP_PlayerCharacter.BP_PlayerStatus` _asbp_player_character)))
  (:`Released`
    (bind _asbp_player_character_2 (cast `/Game/Character/BP_PlayerCharacter` (`self.K2_GetPawn`)))
    (`/Game/BluePrints/Class/BP_PlayerStatus.Owner_StopDash` (`/Game/Character/BP_PlayerCharacter.BP_PlayerStatus` _asbp_player_character_2))))

(event `SetTimerForLineTrace`
  ;[1 1 1] 클라이언트 플레이어 : Line Trace
  (bind _returnvalue (`KismetSystemLibrary.K2_SetTimerDelegate` (delegate `StartLineTrace`) 0.1 true))
  (set `self.TimerHandle` _returnvalue))

(event `StartLineTrace`
  ;[1 1 1] 클라이언트 플레이어 : Line Trace
  (`self.TryPickUpItem`))

(event `ServerSetPlayerName`
  (params (PlayerName :type String))
  ;[1 1 1] 플레이어 이름 설정
  (bind _asbp_player_character (cast `/Game/Character/BP_PlayerCharacter` (`self.K2_GetPawn`)))
  (set `/Game/Character/BP_PlayerCharacter.PlayerName` PlayerName _asbp_player_character))

(event `InputAxis|MoveRight`
  (params (AxisValue :type "Float (single-precision)"))
  ;[1 1 1] 전후좌우 이동
  (bind _asbp_player_character (cast `/Game/Character/BP_PlayerCharacter` (`self.K2_GetPawn`)))
  (`Pawn.AddMovementInput` _asbp_player_character (`.RightVector` (`self.GetDirectionVector`)) AxisValue false))

(event `Server_SaveGUID`
  (params (ItemID :type "Guid Structure"))
  ;[1 1 1] 클라이언트 플레이어 : Line Trace
  ;;[1 1 1] Trace에서 받은 GUID를 저장
  (set `self.ItemID` ItemID))

(event `InputAction|Jump`
  (params (Key :type "Key Structure"))
  ;[1 1 1] 점프
  (:`Pressed`
    (bind _asbp_player_character (cast `/Game/Character/BP_PlayerCharacter` (`self.K2_GetPawn`)))
    (`Character.Jump` _asbp_player_character))
  (:`Released`
    (bind _asbp_player_character_2 (cast `/Game/Character/BP_PlayerCharacter` (`self.K2_GetPawn`)))
    (`Character.StopJumping` _asbp_player_character_2)))

(event `InputAxis|Turn`
  (params (AxisValue :type "Float (single-precision)"))
  ;[1 1 1] 카메라 회전
  (`self.AddYawInput` AxisValue))

(event `InputAxis|LookUp`
  (params (AxisValue :type "Float (single-precision)"))
  ;[1 1 1] 카메라 회전
  (`self.AddPitchInput` AxisValue))

(event `Key|E`
  (params (Key :type "Key Structure"))
  ;[1 1 1] E버튼 : 아이템을 획득할 수 있을 때, 아이템을 획득.
  (:`Pressed`
    (if (`self.CraftMode`)
      (bind _currentcraft (`self.CurrentCraft`)
        (:`then`
          (if (not (`/Game/BluePrints/Object/Craft/BP_BaseCraft.IsProcessing` _currentcraft))
            (bind _asbp_player_character (cast `/Game/Character/BP_PlayerCharacter` (`self.K2_GetPawn`)))
            (`/Game/Character/BP_PlayerCharacter.Owner_CraftBuilding` _asbp_player_character (`self.CurrentCraft`))))
        (:`else`))
      (elif (`self.IsPickUp`)
        (`self.CheckAddItem`)
        (elif (`self.InteractMode`)
          (bind _interactcraft (`self.InteractCraft`)
            (:`then`
              (message `/Game/BluePrints/Class/BPI_Interactable.OnInteract` _interactcraft)
              (bind _asbp_fire (cast `/Game/BluePrints/Object/Craft/BP_Fire` _interactcraft)) ; 해당 건축물이 캠프파이어라면
              (`self.InteractWithFire` _asbp_fire))
            (:`else`
              (`KismetSystemLibrary.PrintString` "건물 없음"))))))))

(event `Key|One`
  (params (Key :type "Key Structure"))
  ;[1 1 1] 1번 버튼 : 도끼 장착, 해제
  (:`Pressed`
    (bind _asbp_player_character (cast `/Game/Character/BP_PlayerCharacter` (`self.K2_GetPawn`)))
    (if (`self.IsEquipTool`)
      (`/Game/Character/BP_PlayerCharacter.Owner_UnEquipTool` _asbp_player_character)
      (set `self.IsEquipTool` false)
      (else
        (`/Game/Character/BP_PlayerCharacter.Owner_EquipTool` _asbp_player_character "NewEnumerator0")
        (set `self.IsEquipTool` true)))))

(event `Key|O`
  (params (Key :type "Key Structure"))
  (bind _asbp_world_hud (`self.GetWorldHUD`))
  ;[1 1 1] O 버튼 : 옵션 버튼
  (:`Pressed`
    (bind _optionui (`/Game/BluePrints/HUD/BP_WorldHUD.OptionUI` _asbp_world_hud)
      (:`then`
        (if (`Widget.IsInViewport` _optionui)
          (`/Game/BluePrints/HUD/BP_WorldHUD.HideOptionUI` _asbp_world_hud)
          (else
            (`/Game/BluePrints/HUD/BP_WorldHUD.ShowOptionUI` _asbp_world_hud :!label _label))))
      (:`else`
        (goto _label)))))

(event `Server_Destroy`
  ;[1 1 1] 서버_ID를 이용해 아이템을 삭제 요청
  (`/Game/BluePrints/Class/BP_ItemManager.DestroyItemFromGUID` (`/Game/BluePrints/GameMode/BP_WorldGM.BP_ItemManager` (`self.GetWorldGM`)) (`self.ItemID`)))

(event `Key|I`
  (params (Key :type "Key Structure"))
  (bind _asbp_world_hud (`self.GetWorldHUD`))
  ;[1 1 1] I 버튼 : 인벤토리 버튼 토글
  (:`Pressed`
    (bind _inventoryui (`/Game/BluePrints/HUD/BP_WorldHUD.InventoryUI` _asbp_world_hud)
      (:`then`
        (if (`Widget.IsInViewport` _inventoryui)
          (`/Game/BluePrints/HUD/BP_WorldHUD.CloseInventory` _asbp_world_hud)
          (else
            (`/Game/BluePrints/HUD/BP_WorldHUD.OpenInventory` _asbp_world_hud :!label _label_2))))
      (:`else`
        (goto _label_2)))))

(event `InputAction|FireAction`
  (params (Key :type "Key Structure"))
  ;[1 1 1] 왼쪽 마우스 버튼 : 도구 사용
  (:`Pressed`
    (bind _asbp_player_character (cast `/Game/Character/BP_PlayerCharacter` (`self.K2_GetPawn`)))
    (`/Game/Character/BP_PlayerCharacter.Owner_ToolAction` _asbp_player_character (`self.CurrentTool`))))

(event `Key|B`
  (params (Key :type "Key Structure"))
  (bind _asbp_world_hud (`self.GetWorldHUD`))
  ;[1 1 1] B버튼 : CraftBook 오픈 / 해제
  (:`Pressed`
    (bind _craftbookui (`/Game/BluePrints/HUD/BP_WorldHUD.CraftBookUI` (`self.GetWorldHUD`)) ; 현재 UI가 유효하다면
      (:`then`
        (if (`Widget.IsInViewport` _craftbookui)
          (`/Game/BluePrints/HUD/BP_WorldHUD.HideCraftBookUI` _asbp_world_hud)
          (else
            (`/Game/BluePrints/HUD/BP_WorldHUD.ShowCraftBookUI` _asbp_world_hud :!label _label_3))))
      (:`else`
        (goto _label_3)))))

(event `Owner_SetPreviewBuilding`
  ;[1 1 1] 프리뷰 메쉬
  (`self.SetPreviewBuilding` (`self.CurrentCraftType`)))

(event `Key|C`
  (params (Key :type "Key Structure"))
  ;[1 1 1] C 버튼 : 프리뷰 메시 건설 확정
  (:`Pressed`
    (if (`self.IsSetPreview`)
      (`self.Owner_DestroyPreviewBuilding`)
      (`self.Owner_SetPreviewCraft` (`self.CurrentCraftType`) (`self.PreviewTransform`))
      (`/Game/BluePrints/HUD/BP_WorldHUD.HidePreviewIcon` (`self.GetWorldHUD`)))))

(event `Owner_DestroyPreviewBuilding`
  ;[1 1 1] 프리뷰 메쉬
  (`KismetSystemLibrary.K2_ClearAndInvalidateTimerHandle` (`self.PreviewTH`))
  (bind _previewactor (`self.PreviewActor`)
    (:`then`
      (`self.K2_DestroyActor` _previewactor) ; 클라 : 프리뷰 메쉬 제거
      (`KismetSystemLibrary.PrintString` "삭제완료"))
    (:`else`)))

(event `Owner_SetPreviewCraft`
  (params (BuildingType :type "/Game/Enums/E_Craft Enum" :default "NewEnumerator0") (Tranform :type "Transform Structure"))
  ;[1 1 1] C 버튼 : 프리뷰 메시 건설 확정
  (`self.Server_SetPreviewCraft` BuildingType Tranform))

(event `Server_SetPreviewCraft`
  (params (BuildingType :type "/Game/Enums/E_Craft Enum" :default "NewEnumerator0") (Tranform :type "Transform Structure"))
  ;[1 1 1] C 버튼 : 프리뷰 메시 건설 확정
  (`/Game/BluePrints/Class/BP_CraftManager.SpawnGhostCraft` (`/Game/BluePrints/GameMode/BP_WorldGM.BP_CraftManager` (`self.GetWorldGM`)) BuildingType Tranform))

(event `Key|X`
  (params (Key :type "Key Structure"))
  ;[1 1 1] X 버튼 : 건물 설치 취소
  (:`Pressed`
    (if (`self.IsSetPreview`)
      (`self.Owner_DestroyPreviewBuilding`)
      (`/Game/BluePrints/HUD/BP_WorldHUD.HidePreviewIcon` (`self.GetWorldHUD`))
      (set `self.IsSetPreview` false))))

(event `Owner_SetCraftUI`
  (params (CurrentCraft :type "/Game/BluePrints/Object/Craft/BP_BaseCraft Object Reference"))
  (`self.SetCraftMode` CurrentCraft))

(event `Server_FireON`
  (params (Actor :type "/Game/BluePrints/Object/Craft/BP_Fire Object Reference"))
  (`/Game/BluePrints/Object/Craft/BP_Fire.Server_OnFire` Actor))

(event `Owner_HidCraftUI`
  (`self.HideCraftMode`))

(fn `CanPickUpItem`
  (params (HitActor :type "Actor Object Reference"))
  ;[1 1 1] 충돌된 객체가 획득가능한 아이템인지 판별
  (`/Engine/EditorBlueprintResources/StandardMacros.IsValid` HitActor ; 충돌된 객체가 유효한지
    (:`Is Valid`
      (bind _asbp_player_character (cast `/Game/Character/BP_PlayerCharacter` (`self.K2_GetPawn`)))
      (bind (_itemid _itemst) (`/Game/BluePrints/Class/BP_PlayerInventory.GetItemIDFromActor` (`/Game/Character/BP_PlayerCharacter.BP_PlayerInventory` _asbp_player_character) HitActor))
      (set `self.ItemStruct` _itemst)
      (`self.Server_SaveGUID` _itemid)
      (set `self.IsPickUp` true) ; 현재 아이템을 먹을 수 있도록 설정.
      (`self.SetPickUpItemUI`) ; IsPickUp 상태에 따라 UI 표시 전환
    )
    (:`Is Not Valid`
      (`KismetSystemLibrary.PrintString` "유효하지 않음"))))

(fn `CheckAddItem`
  (locals (IsAdd :type Boolean))
  ;[1 1 1] 현재 아이템을 얻을 수 있는 상태인지 확인
  (bind _asbp_player_character (cast `/Game/Character/BP_PlayerCharacter` (`self.K2_GetPawn`)))
  (bind _bp_playerinventory (`/Game/Character/BP_PlayerCharacter.BP_PlayerInventory` _asbp_player_character))
  (bind _isadd (`/Game/BluePrints/Class/BP_PlayerInventory.CheckIsGetItem` _bp_playerinventory (`self.ItemStruct`))) ; 아이템을 얻을 수 있는 상태인지 확인
  (if _isadd
    (`/Game/BluePrints/Class/BP_PlayerInventory.OwnerAddItemToInven` _bp_playerinventory (`self.ItemStruct`)) ; 아이템 추가
    (`self.Server_Destroy`) ; 오브젝트 삭제
    (else
      (`KismetSystemLibrary.PrintString` "아이템을 얻을 수 없음"))))

(fn `FireActionWithTool`
  (params (Selection :type "/Game/Enums/E_Tool Enum" :default "NewEnumerator0")))

(fn `GetForwardVector`
  (params (InputPin :type "Float (double-precision)"))
  (returns (StartPoint :type "Vector Structure") (EndPoint :type "Vector Structure"))
  ;[1 1 1] Line Trace를 위한 Forward Line 구하기
  (bind _asbp_player_character (cast `/Game/Character/BP_PlayerCharacter` (`self.K2_GetPawn`)))
  (bind _camera (`/Game/Character/BP_PlayerCharacter.Camera` _asbp_player_character))
  (bind _returnvalue (`SceneComponent.K2_GetComponentLocation` _camera))
  (return _returnvalue (+ _returnvalue (* (`KismetMathLibrary.GetForwardVector` (`SceneComponent.K2_GetComponentRotation` _camera)) InputPin))))

(fn `GetPlayerName`
  (returns (PlayerName :type String))
  (bind _asbp_multi_forest_gi (cast `/Game/BluePrints/BP_MultiForestGI` (`GameplayStatics.GetGameInstance`)))
  (return (`/Game/BluePrints/BP_MultiForestGI.PlayerName` _asbp_multi_forest_gi)))

(fn `GetPreviewBuilding`
  (params (CraftType :type "/Game/Enums/E_Craft Enum" :default "NewEnumerator0"))
  (returns (Class :type "Actor Class Reference"))
  (locals (ActorClass :type "Actor Class Reference"))
  (switch `/Game/Enums/E_Craft` CraftType
    (:`NewEnumerator0`
      (set `local.ActorClass` "/Game/BluePrints/Object/Craft/BP_GhostShelter.BP_GhostShelter_C"))
    (:`NewEnumerator1`
      (set `local.ActorClass` "/Game/BluePrints/Object/Craft/BP_GhostFire.BP_GhostFire_C")))
  (return (`local.ActorClass`)))

(fn `HideCraftMode`
  (locals (WorldHUD :type "/Game/BluePrints/HUD/BP_WorldHUD Object Reference"))
  (bind _output_get (set `local.WorldHUD` (`self.GetWorldHUD`)))
  (`/Game/BluePrints/HUD/BP_WorldHUD.HideCraftModeUI` _output_get))

(fn `InteractWithFire`
  (params (Craft :type "/Game/BluePrints/Object/Craft/BP_Fire Object Reference"))
  (if (not (`/Game/BluePrints/Object/Craft/BP_Fire.IsFireOn` Craft))
    (`self.Server_FireON` Craft)
    (set `/Game/BluePrints/Object/Craft/BP_Fire.IsFireOn` true (`local.Craft`))))

(fn `OnRep_CurrentCraft`
  (`/Engine/EditorBlueprintResources/ActorMacros.Switch Has Authority` ; 클라에서 실행
    (:`Remote`
      (bind _currentcraft (`self.CurrentCraft`)
        (:`then`
          (bind _craftmodeui (`/Game/BluePrints/HUD/BP_WorldHUD.CraftModeUI` (`self.GetWorldHUD`))
            (:`then`
              (set `/Game/UIWidget/Craft/WBP_CraftMode.CurrentCraft` _currentcraft _craftmodeui))
            (:`else`)))
        (:`else`)))))

(fn `PerformLineTrace`
  (returns (IsHit :type Boolean) (HitActor :type "Actor Object Reference"))
  (locals (LineTraceValue :type "Float (double-precision)" :default 500.0))
  (bind (_startpoint _endpoint) (`self.GetForwardVector` (`local.LineTraceValue`)))
  ;[1 1 1] LineTrace로 아이템 감지
  (bind _outhit (`KismetSystemLibrary.LineTraceSingle` _startpoint _endpoint "TraceTypeQuery1"))
  (bind (_bblockinghit _binitialoverlap _time _distance _location _impactpoint _normal _impactnormal _physmat _hitactor) (`GameplayStatics.BreakHitResult` _outhit))
  (return _bblockinghit _hitactor))

(fn `SetCraftMode`
  (params (CurrentCraft :type "/Game/BluePrints/Object/Craft/BP_BaseCraft Object Reference"))
  (locals (WorldHUD :type "/Game/BluePrints/HUD/BP_WorldHUD Object Reference"))
  (set `self.CraftMode` true)
  (if (not (`self.HasAuthority`))
    (`KismetSystemLibrary.PrintString` "건축물 노티파이")
    (`/Game/BluePrints/HUD/BP_WorldHUD.ShowCraftModeUI` (`self.GetWorldHUD`) (`local.CurrentCraft`))))

(fn `SetPickUpItemUI`
  (locals (WorldHUD :type "/Game/BluePrints/HUD/BP_WorldHUD Object Reference"))
  ;[1 1 1] IsPickUp에 따른 함수 실행 / 현재 아이템 획득이 가능한가
  (set `local.WorldHUD` (`self.GetWorldHUD`))
  (if (`self.IsPickUp`)
    (`/Game/BluePrints/HUD/BP_WorldHUD.Show Pick Up Item` (`local.WorldHUD`))
    (else
      (`/Game/BluePrints/HUD/BP_WorldHUD.HidePickUpItem` (`local.WorldHUD`)))))

(fn `SetPreviewBuilding`
  (params (BuildingType :type "/Game/Enums/E_Craft Enum" :default "NewEnumerator0"))
  (locals (LineTraceValue :type "Float (double-precision)" :default 1000.0) (CheckObject :type "Array of EObjectTypeQuery Enum") (Location :type "Vector Structure"))
  (bind _previewactor (`self.PreviewActor`))
  (bind (_startpoint _endpoint) (`self.GetForwardVector` (`local.LineTraceValue`)))
  ;[1 1 1] 건물의 프리뷰 액터 생성 : 건물을 설치할 수 있는지 없는지 확인하며 설치할 장소 물색
  (bind _outhit (`KismetSystemLibrary.LineTraceSingle` _startpoint _endpoint "TraceTypeQuery1")) ; 라인 트레이스 실행
  (bind (_bblockinghit _binitialoverlap _time _distance _location) (`GameplayStatics.BreakHitResult` _outhit))
  (set `local.Location` _location)
  (if (not (`KismetSystemLibrary.IsValid` (`self.PreviewActor`)))
    (bind _returnvalue (`|SpawnActorFromClass` (`self.GetPreviewBuilding` (`local.BuildingType`)) (`KismetMathLibrary.Conv_VectorToTransform` _location) "AlwaysSpawn" "OverrideRootScale" null null)) ; 없다면 생성
    (`KismetSystemLibrary.PrintString` "스폰완료")
    (bind _output_get (set `self.PreviewActor` (cast `/Game/BluePrints/Object/Craft/BP_BaseCraft` _returnvalue :!pure true))))
  (bind _outactors (`KismetSystemLibrary.SphereOverlapActors` (`local.Location`) (`/Game/BluePrints/Object/Craft/BP_BaseCraft.CollisionSize` _output_get) (`local.CheckObject`) null (`|MakeArray` (`self.K2_GetPawn`) null :!type "Actor Object Reference"))) ; 해당 위치에서 액터 오버랩을 실행
  (bind _output_get_2 (set `self.IsSetPreview` (== (`KismetArrayLibrary.Array_Length` _outactors) 0)))
  (if _output_get_2
    (`/Game/BluePrints/Object/Craft/BP_BaseCraft.SetPreviewColor` (`self.PreviewActor`) (`self.IsSetPreview`)) ; 설치가능함 : 녹색으로 색깔 처리
    (else
      (`/Game/BluePrints/Object/Craft/BP_BaseCraft.SetPreviewColor` (`self.PreviewActor`) (`self.IsSetPreview`))))
  (`self.K2_SetActorLocation` (`self.PreviewActor`) (`local.Location`) false false) ; 색깔 변화시킨 뒤, 해당 장소로 프리뷰 액터 위치 설정
  (`self.K2_SetActorRotation` _previewactor (`KismetMathLibrary.MakeRotator` 0.0 0.0 (.yaw (`KismetMathLibrary.FindLookAtRotation` (`self.K2_GetActorLocation` (`self.PreviewActor`)) (`SceneComponent.K2_GetComponentLocation` (`Actor.RootComponent` (`self.K2_GetPawn`)))))) false) ; 프리뷰 액터의 회전값 설정
  (set `self.PreviewTransform` (`self.GetTransform` _previewactor)))

(fn `StartSetPreviewBuilding`
  ;[1 1 1] 프리뷰 메쉬를 사용한 건물 설치 시작
  (set `self.IsSetPreview` false)
  (bind _returnvalue (`KismetSystemLibrary.K2_SetTimer` null "Owner_SetPreviewBuilding" 0.01 true))
  (set `self.PreviewTH` _returnvalue))

(fn `TryPickUpItem`
  (locals (ItemTag :type Name :default "Item") (CraftTag :type Name :default "Craft") (HitActor :type "Actor Object Reference"))
  ;[1 1 1] 아이템 획득 과정
  (bind (_ishit _hitactor) (`self.PerformLineTrace`)) ; 0.3초 마다 Line Trace 발생
  (set `local.HitActor` _hitactor)
  (if _ishit
    (if (`self.ActorHasTag` (`local.HitActor`) (`local.ItemTag`))
      (`self.CanPickUpItem` (`local.HitActor`)) ; 아이템을 얻을 수 있도록
      (else
        ;;[0 0.1085 0.5469] 건축물 상호작용 모드
        (set `self.IsPickUp` false) ; 충돌이 없다면 IsPickUp False + UI 변화
        (`self.SetPickUpItemUI`)
        (if (and (`self.ActorHasTag` (`local.HitActor`) (`local.CraftTag`)) (`KismetSystemLibrary.DoesImplementInterface` (`local.HitActor`) "/Game/BluePrints/Class/BPI_Interactable.BPI_Interactable_C"))
          (set `self.InteractCraft` (`local.HitActor`))
          (set `self.InteractMode` true)
          (else
            (set `self.InteractMode` false)))))
    (else
      (set `self.IsPickUp` false) ; 충돌이 없다면 IsPickUp False + UI 변화
      (set `self.InteractMode` false)
      (`self.SetPickUpItemUI`))))

(fn `UserConstructionScript`
  (`parent.UserConstructionScript`))