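; BP_BasePC is a base Player Controller Blueprint that provides typed getters for the game's World framework objects and game instance.
; Functions cast the player state, game mode, HUD, game state and game instance to their project Blueprint classes.
; The game mode getter resolves only with authority, matching its server-only existence.
; A failed HUD cast prints a Korean debug message, while the other failed casts return nothing silently.
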(fn `Get World PS`
  (returns (`AsBP World PS` :type "/Game/BluePrints/PlayerState/BP_WorldPS Object Reference"))
  (bind _asbp_world_ps (cast `/Game/BluePrints/PlayerState/BP_WorldPS` (`self.PlayerState`)))
  (return _asbp_world_ps))

(fn `GetMultiForestInstance`
  (returns (`AsBP Multi Forest GI` :type "/Game/BluePrints/BP_MultiForestGI Object Reference"))
  (bind _asbp_multi_forest_gi (cast `/Game/BluePrints/BP_MultiForestGI` (`GameplayStatics.GetGameInstance`)))
  (return _asbp_multi_forest_gi))

(fn `GetWorldGM`
  (returns (`AsBP World GM` :type "/Game/BluePrints/GameMode/BP_WorldGM Object Reference"))
  (`/Engine/EditorBlueprintResources/ActorMacros.Switch Has Authority`
    (:`Authority`
      (bind _asbp_world_gm (cast `/Game/BluePrints/GameMode/BP_WorldGM` (`GameplayStatics.GetGameMode`)))
      (return _asbp_world_gm))))

(fn `GetWorldGS`
  (returns (`AsBP World GS` :type "/Game/BluePrints/GameState/BP_WorldGS Object Reference"))
  (bind _asbp_world_gs (cast `/Game/BluePrints/GameState/BP_WorldGS` (`GameplayStatics.GetGameState`)))
  (return _asbp_world_gs))

(fn `GetWorldHUD`
  (returns (`AsBP World HUD` :type "/Game/BluePrints/HUD/BP_WorldHUD Object Reference"))
  (bind _asbp_world_hud (cast `/Game/BluePrints/HUD/BP_WorldHUD` (`self.GetHUD`))
    (:`then`
      (return _asbp_world_hud))
    (:`CastFailed`
      (`KismetSystemLibrary.PrintString` "HUD 못가져옴"))))

(fn `UserConstructionScript`)