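; BP_BaseCraft is a base Blueprint for a craftable building that tracks the ingredients gathered toward its recipe.
; A data table row sets the recipe and seeds CurrentIngredient, which PlusCount fills up to each required amount and CheckItemArray tests for completion.
; On clients, trigger overlaps show or hide the player controller's craft UI, and CurrentIngredient's RepNotify refreshes it in craft mode.
; SetPreviewColor tints the preview materials green or red.
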(event OnComponentBeginOverlap(Trigger)
  (params (OverlappedComponent :type Primitive%20Component%20Object%20Reference) (OtherActor :type Actor%20Object%20Reference) (OtherComp :type Primitive%20Component%20Object%20Reference) (OtherBodyIndex :type Integer) (bFromSweep :type Boolean) (SweepResult :type Hit%20Result%20Structure%20%28by%20ref%29))
  (bind _self self)
  ;[1 1 1] Trigger 이벤트
  (Networking|SwitchHasAuthority
    (:Remote
      (bind _asbp_player_character (Utilities|Casting|CastToBP_PlayerCharacter OtherActor))
      (Variables|Default|SetAs%20BP%20Player%20Character _asbp_player_character)
      (bind _asbp_world_pc (Utilities|Casting|CastToBP_WorldPC (Pawn|GetController _asbp_player_character)))
      (Variables|/Game/BluePrints/PlayerController/BP_WorldPC.BP_WorldPC_C|SetCurrentCraft _asbp_world_pc _self)
      (Default|OwnerSetCraftUI _asbp_world_pc _self))))

(event OnComponentEndOverlap(Trigger)
  (params (OverlappedComponent :type Primitive%20Component%20Object%20Reference) (OtherActor :type Actor%20Object%20Reference) (OtherComp :type Primitive%20Component%20Object%20Reference) (OtherBodyIndex :type Integer))
  ;[1 1 1] Trigger 이벤트
  (Networking|SwitchHasAuthority
    (:Remote
      (bind _asbp_player_character (Utilities|Casting|CastToBP_PlayerCharacter OtherActor))
      (bind _asbp_world_pc (Utilities|Casting|CastToBP_WorldPC (Pawn|GetController _asbp_player_character)))
      (Variables|/Game/BluePrints/PlayerController/BP_WorldPC.BP_WorldPC_C|SetCraftMode _asbp_world_pc false) ; 크래프트 모드 해제
      (Default|OwnerHidCraftUI _asbp_world_pc))))

(fn ConstructionScript)

(fn SetPreviewColor
  (params (Condition :type Boolean))
  ;[1 1 1] Preview Mesh Color Setting
  (if Condition
    (for _array_element (Variables|Default|GetMeshMaterials)
      (Rendering|Material|SetVectorParameterValue _array_element "BaseColor" "(R=0.000000,G=1.000000,B=0.000000,A=1.000000)" :!class /Script/Engine.MaterialInstanceDynamic))
    (else
      (for _array_element_2 (Variables|Default|GetMeshMaterials)
        (Rendering|Material|SetVectorParameterValue _array_element_2 "BaseColor" "(R=1.000000,G=0.000000,B=0.000000,A=1.000000)" :!class /Script/Engine.MaterialInstanceDynamic)))))

(fn CheckItemArray
  ;[1 1 1] Comment
  (for (_array_element _array_index) (Variables|Default|GetCurrentIngredient)
    (if (not (and (== (.Quantity (Utilities|Struct|BreakDS_ItemRecipe _array_element)) (.Quantity (Utilities|Struct|BreakDS_ItemRecipe (Utilities|Array|Get(acopy) (Variables|Default|GetCraftRecipe) _array_index)))) (Utilities|Enum|Equal(Enum) (.ItemType (Utilities|Struct|BreakDS_ItemRecipe _array_element)) (.ItemType (Utilities|Struct|BreakDS_ItemRecipe (Utilities|Array|Get(acopy) (Variables|Default|GetCraftRecipe) _array_index))))))
      (return false) ; 플레이어의 재료 배열에서\n재료가 다 모아지지 않았음
    ))
  (Development|PrintString "모든 재료가 다 모아짐")
  (return true) ; 플레이어의 재료 배열에서\n재료가 다 모아지지 않았음
)

(fn SetCraftRecipe
  (params (RowName :type Name))
  (bind _returnvalue (Utilities|GetDataTableRow "/Game/DataTable/DT_CraftRecipe.DT_CraftRecipe" RowName) ; 데이터 테이블에서 RowName으로 레시피 정보를 가져온다.
    (:then
      (Variables|Default|SetCraftType (.CraftType (Utilities|Struct|BreakDS_Crafting _returnvalue)))
      (bind _output_get (Variables|Default|SetCraftRecipe (.Ingredient (Utilities|Struct|BreakDS_Crafting _returnvalue))))
      (for _array_element _output_get
        (Development|PrintString (Utilities|String|EnumtoString (.ItemType (Utilities|Struct|BreakDS_ItemRecipe _array_element))))
        (Utilities|Array|Add (Variables|Default|GetCurrentIngredient) (Utilities|Struct|MakeDS_ItemRecipe 0 (.ItemType (Utilities|Struct|BreakDS_ItemRecipe _array_element))))))))

(fn PlusCount
  (params (ItemType :type E_ItemType%20Enum :default "NewEnumerator0"))
  ;[1 1 1] Comment
  (for (_array_element _array_index) (Variables|Default|GetCurrentIngredient)
    (bind _output_get (LocalVariables|SetItemRecipe _array_element))
    (if (and (Utilities|Enum|Equal(Enum) (.ItemType (Utilities|Struct|BreakDS_ItemRecipe _output_get)) ItemType) (< (.Quantity (Utilities|Struct|BreakDS_ItemRecipe _output_get)) (.Quantity (Utilities|Struct|BreakDS_ItemRecipe (Utilities|Array|Get(acopy) (Variables|Default|GetCraftRecipe) _array_index)))))
      (Math|Integer|IncrementInt (.Quantity (Utilities|Struct|BreakDS_ItemRecipe _output_get))
        (:%20%20
          (Utilities|Array|SetArrayElem (Variables|Default|GetCurrentIngredient) _array_index (LocalVariables|GetItemRecipe))
          (return))))))

(fn OnRepCurrentIngredient
  ;[1 1 1] Comment
  (Networking|SwitchHasAuthority
    (:Remote
      (bind _as_bp_player_character (Variables|Default|GetAs%20BP%20Player%20Character)
        (:then
          (bind _asbp_world_pc (Utilities|Casting|CastToBP_WorldPC (Pawn|GetController _as_bp_player_character)))
          (if (and (Variables|/Game/BluePrints/PlayerController/BP_WorldPC.BP_WorldPC_C|GetCraftMode _asbp_world_pc) (stale _bsuccess))
            (Default|UpdateCraftModeUI (Default|GetWorldHUD _asbp_world_pc) self)))
        (:else
          (Development|PrintString "캐릭터 유효하지 않음"))))))