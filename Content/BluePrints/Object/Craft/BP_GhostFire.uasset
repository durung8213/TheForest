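; BP_GhostFire is a craft object Blueprint that sets up a ghostly preview of a fire.
; On BeginPlay it creates dynamic instances of M_GhostMaterial on three static meshes and collects them in MeshMaterials.
; It then sets the collision size used for overlap checks and loads its craft recipe by RowName through SetCraftRecipe.
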(event `self.ReceiveBeginPlay`
  (bind _returnvalue (`PrimitiveComponent.CreateDynamicMaterialInstance` (`self.StaticMesh`) 0 "/Game/ExportForest/Material/M_GhostMaterial.M_GhostMaterial" "None"))
  (`KismetArrayLibrary.Array_Add` (`self.MeshMaterials`) _returnvalue)
  (bind _returnvalue_2 (`PrimitiveComponent.CreateDynamicMaterialInstance` (`self.StaticMesh1`) 0 "/Game/ExportForest/Material/M_GhostMaterial.M_GhostMaterial" "None"))
  (`KismetArrayLibrary.Array_Add` (`self.MeshMaterials`) _returnvalue_2)
  (bind _returnvalue_3 (`PrimitiveComponent.CreateDynamicMaterialInstance` (`self.StaticMesh2`) 0 "/Game/ExportForest/Material/M_GhostMaterial.M_GhostMaterial" "None"))
  (`KismetArrayLibrary.Array_Add` (`self.MeshMaterials`) _returnvalue_3)
  (set `self.CollisionSize` 50.0) ; 이 사이즈 만큼  Overlap 실행
  (`self.SetCraftRecipe` (`self.RowName`)))

(fn `UserConstructionScript`
  (`parent.UserConstructionScript`))