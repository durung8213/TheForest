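; BP_Fire is a campfire interactable that serves as a cooking station once lit.
; Its trigger tracks overlap and caches the player; interacting toggles the cooking UI through the world HUD, opening the inventory and switching input mode and cursor.
; A server event calls a multicast to activate fire particles and set IsFireOn, which gates opening the UI.
; ProcessingCook and the IsInCampFire RepNotify are unfinished stubs with no effect.
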(event `self.FireTrigger.OnComponentBeginOverlap`
  (params (OverlappedComponent :type "PrimitiveComponent Object Reference") (OtherActor :type "Actor Object Reference") (OtherComp :type "PrimitiveComponent Object Reference") (OtherBodyIndex :type Integer) (bFromSweep :type Boolean) (SweepResult :type "HitResult Structure (by ref)"))
  ;[1 1 1] Comment
  (set `self.IsInCampFire` true)
  (`KismetSystemLibrary.PrintString` "InFire")
  (bind _asbp_player_character (cast `/Game/Character/BP_PlayerCharacter` OtherActor))
  (set `self.Player` _asbp_player_character))

(event `self.FireTrigger.OnComponentEndOverlap`
  (params (OverlappedComponent :type "PrimitiveComponent Object Reference") (OtherActor :type "Actor Object Reference") (OtherComp :type "PrimitiveComponent Object Reference") (OtherBodyIndex :type Integer))
  ;[1 1 1] Comment
  (set `self.IsInCampFire` false)
  (`KismetSystemLibrary.PrintString` "OutFire"))

(event `self.OnInteract`
  (`self.InteractCampfire`))

(event `Server_OnFire`
  ;[1 1 1] Comment
  (`self.Multi_OnFire`))

(event `Multi_OnFire`
  ;[1 1 1] Comment
  (`ActorComponent.SetActive` (`self.ParticleSystem`) true false)
  (`KismetSystemLibrary.PrintString` "파티클 온")
  (set `self.IsFireOn` true))

(fn `InteractCampfire`
  (locals (PlayerController :type "/Game/BluePrints/PlayerController/BP_WorldPC Object Reference"))
  (bind _asbp_world_hud (`/Game/BluePrints/PlayerController/BP_BasePC.GetWorldHUD` (`local.PlayerController`)))
  ;[1 1 1] Comment
  (bind _player (`self.Player`)
    (:`then`
      (bind _asbp_world_pc (cast `/Game/BluePrints/PlayerController/BP_WorldPC` (`Pawn.GetController` _player)))
      (set `local.PlayerController` _asbp_world_pc)
      (bind _asbp_world_hud_2 (`/Game/BluePrints/PlayerController/BP_BasePC.GetWorldHUD` _asbp_world_pc))
      (bind _campfireui (`/Game/BluePrints/HUD/BP_WorldHUD.CampFireUI` _asbp_world_hud_2)
        (:`then`
          (if (`Widget.IsInViewport` _campfireui)
            (`WidgetBlueprintLibrary.SetInputMode_GameOnly` (`local.PlayerController`))
            (`/Game/BluePrints/HUD/BP_WorldHUD.HideCookingUI` _asbp_world_hud_2)
            (set `PlayerController.bShowMouseCursor` false (`local.PlayerController`))
            (else
              (if (`self.IsFireOn`) :!label _label
                ;;[1 1 1] 요리 가능한 상태 : UI 실행
                (bind _inventoryui (`/Game/BluePrints/HUD/BP_WorldHUD.InventoryUI` _asbp_world_hud)
                  (:`then`
                    (if (not (`Widget.IsInViewport` _inventoryui))
                      (`/Game/BluePrints/HUD/BP_WorldHUD.OpenInventory` _asbp_world_hud :!label _label_2)))
                  (:`else`
                    (goto _label_2)))
                (`/Game/BluePrints/HUD/BP_WorldHUD.ShowCookingUI` _asbp_world_hud)
                (`WidgetBlueprintLibrary.SetInputMode_GameAndUIEx` (`local.PlayerController`) null)
                (set `PlayerController.bShowMouseCursor` true (`local.PlayerController`))))))
        (:`else`
          (goto _label))))
    (:`else`
      (`KismetSystemLibrary.PrintString` "1"))))

(fn `OnRep_IsInCampFire`
  (if (`self.IsInCampFire`)
    (`/Engine/EditorBlueprintResources/ActorMacros.Switch Has Authority`
      (:`Remote`
        (bind _asbp_player_character (cast `/Game/Character/BP_PlayerCharacter` (`GameplayStatics.GetPlayerPawn` 0)))
        (cast `/Game/BluePrints/PlayerController/BP_WorldPC` (`Pawn.GetController` _asbp_player_character))))))

(fn `ProcessingCook`
  (for _ (`self.Ingredient`)
    _))

(fn `ShowCookingUI`
  (bind _asbp_world_pc (cast `/Game/BluePrints/PlayerController/BP_WorldPC` (`Pawn.GetController` (`self.Player`)))
    (:`then`
      (`/Game/BluePrints/HUD/BP_WorldHUD.ShowCookingUI` (`/Game/BluePrints/PlayerController/BP_BasePC.GetWorldHUD` _asbp_world_pc))
      (`WidgetBlueprintLibrary.SetInputMode_GameAndUIEx` _asbp_world_pc null)
      (set `PlayerController.bShowMouseCursor` true _asbp_world_pc))
    (:`CastFailed`
      (`KismetSystemLibrary.PrintString` "컨트롤러 변환 실패"))))

(fn `UserConstructionScript`
  (`parent.UserConstructionScript`))