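; Base tree Blueprint that turns a tree into a wood item in the world.
; An owner event forwards to a server event, which runs SpawnWoodItem through the BP_WorldGM game mode.
; That function has the item manager spawn the item at the tree's transform, then destroy the tree by TreeID.
; A separate SpawnWoodEmitter function plays an explosion particle there, but nothing in this graph calls it.
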(event `Owner_SpawnWoodItem`
  ;[1 1 1] 나무 아이템 생성
  (`self.Server_SpawnWoodItem`))

(event `Server_SpawnWoodItem`
  ;[1 1 1] 나무 아이템 생성
  (`self.SpawnWoodItem`))

(fn `SpawnWoodEmitter`
  (bind (_returnvalue_location _returnvalue_rotation _returnvalue_scale) (`KismetMathLibrary.BreakTransform` (`SceneComponent.K2_GetComponentToWorld` (`self.Scene`))))
  (`GameplayStatics.SpawnEmitterAtLocation` "/Game/StarterContent/Particles/P_Explosion.P_Explosion" _returnvalue_location _returnvalue_rotation _returnvalue_scale))

(fn `SpawnWoodItem`
  ;[1 1 1] Comment
  (bind _asbp_world_gm (cast `/Game/BluePrints/GameMode/BP_WorldGM` (`GameplayStatics.GetGameMode`)))
  (`/Game/BluePrints/Class/BP_ItemManager.Server_SpawnNewItem` (`/Game/BluePrints/GameMode/BP_WorldGM.BP_ItemManager` _asbp_world_gm) "NewEnumerator1" (`SceneComponent.K2_GetComponentToWorld` (`self.Scene`)))
  (`/Game/BluePrints/Class/BP_ItemManager.DestroyTreeFromGUID` (`/Game/BluePrints/GameMode/BP_WorldGM.BP_ItemManager` _asbp_world_gm) (`self.TreeID`)))

(fn `UserConstructionScript`)