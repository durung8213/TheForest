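; BP_WorldGM is the world game mode that populates the level and sets up joining players.
; BeginPlay has BPItemManager spawn items, trees and nature, then spawns zombies at every AI spawn point, tracked by GUID in NPCMap for drop-and-destroy removal.
; PostLogin spawns and possesses a character at a PlayerStart, then requests the player's name.
; CheckItemType's crafting ingredient check and build logic is disconnected from its entry.
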(event `self.ReceiveBeginPlay`
  (`parent.ReceiveBeginPlay`)
  (`KismetSystemLibrary.PrintString` "BeginPlay 성공")
  (`/Game/BluePrints/Class/BP_ItemManager.SpawnItemFromGUID` (`self.BP_ItemManager`))
  (`/Game/BluePrints/Class/BP_ItemManager.SpawnTreeFromGUID` (`self.BP_ItemManager`))
  (`/Game/BluePrints/Class/BP_ItemManager.SpawnNatureList` (`self.BP_ItemManager`))
  (`self.SpawnAIList`) ; AI NPC 스폰
)

(event `self.K2_PostLogin`
  (params (NewPlayer :type "PlayerController Object Reference"))
  (`KismetSystemLibrary.PrintString` "OnPostLogin 성공")
  (bind _asbp_world_pc (cast `/Game/BluePrints/PlayerController/BP_WorldPC` NewPlayer)
    (:`then`
      (set `self.World PC` _asbp_world_pc)
      (`|ExecutionSequence`
        (:`then_0`
          (`self.SetPlayer` (`self.World PC`)) ; 플레이어 설정
        )
        (:`then_1`
          (`/Game/BluePrints/PlayerController/BP_WorldPC.OwnerGetName` (`self.World PC`)) ; 입력받은 이름 설정
        )))
    (:`CastFailed`
      (`KismetSystemLibrary.PrintString` "PlayerController : 형변환 실패"))))

(fn `Check Item Type`
  (params (craft :type "/Game/BluePrints/Object/Craft/BP_BaseCraft Object Reference"))
  (returns (ItemType :type "/Game/Enums/E_ItemType Enum"))
  ;[1 1 1] Comment
)

(fn `Destroy AINPC`
  (params (Key :type "Guid Structure (by ref)"))
  (bind _npcmap (`self.NPCMap`))
  (bind (_value _returnvalue) (`BlueprintMapLibrary.Map_Find` _npcmap Key))
  (if _returnvalue
    (`/Game/Character/BP_AIZombie.Owner_SpawnItem` _value)
    (`self.K2_DestroyActor` _value)
    (`BlueprintMapLibrary.Map_Remove` _npcmap (`local.Key`))
    (else
      (`KismetSystemLibrary.PrintString` "해당되는 NPC 없음"))))

(fn `SetNameUI`
  (params (pName :type String))
  (`KismetSystemLibrary.PrintString` "SetNameUI 접속")
  (bind _asbp_player_character (cast `/Game/Character/BP_PlayerCharacter` (`GameplayStatics.GetPlayerPawn` 0))
    (:`then`
      (`TextRenderComponent.K2_SetText` (`/Game/Character/BP_PlayerCharacter.NickName` _asbp_player_character) (`KismetTextLibrary.Conv_StringToText` (`local.pName`))))
    (:`CastFailed`
      (`KismetSystemLibrary.PrintString` "캐릭터 형변환 실패"))))

(fn `SetPlayer`
  (params (PlayerPC :type "PlayerController Object Reference"))
  ;[1 1 1] 플레이어 생성
  (bind _returnvalue (`GameplayStatics.GetActorOfClass` "/Script/Engine.PlayerStart"))
  (`/Engine/EditorBlueprintResources/StandardMacros.IsValid` _returnvalue
    (:`Is Valid`
      (bind _returnvalue_2 (`|SpawnActorFromClass` "/Game/Character/BP_PlayerCharacter.BP_PlayerCharacter_C" (`self.GetTransform` _returnvalue) "Undefined" "OverrideRootScale" PlayerPC null))
      (`/Engine/EditorBlueprintResources/StandardMacros.IsValid` _returnvalue_2
        (:`Is Valid`
          (`Controller.Possess` PlayerPC _returnvalue_2)
          (`KismetSystemLibrary.PrintString` "Player Possess"))))))

(fn `SpawnAIList`
  (bind _outactors (`GameplayStatics.GetAllActorsOfClass` "/Game/AI/BP_AISpawnPoint.BP_AISpawnPoint_C"))
  (for _array_element _outactors
    (`self.SpawnAINPC` _array_element)))

(fn `SpawnAINPC`
  (params (Point :type "Actor Object Reference"))
  (for _ (range 4)
    (bind _returnvalue (`|SpawnActorFromClass` "/Game/Character/BP_AIZombie.BP_AIZombie_C" (`KismetMathLibrary.Conv_VectorToTransform` (`self.K2_GetActorLocation` Point)) "AlwaysSpawn" "OverrideRootScale" null null))
    (bind _output_get (set `/Game/Character/BP_AIZombie.ZombieID` (`KismetGuidLibrary.NewGuid`) _returnvalue))
    (`BlueprintMapLibrary.Map_Add` (`self.NPCMap`) _output_get _returnvalue)))

(fn `UserConstructionScript`
  (`parent.UserConstructionScript`))