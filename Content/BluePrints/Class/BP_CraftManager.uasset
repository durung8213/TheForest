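; BP_CraftManager spawns and destroys craftable structures (shelter, campfire) and their ghost versions, which are meant to appear for all players.
; Lookup functions map a craft type to its real or ghost class, which is always spawned regardless of collision.
; Separate GUID-keyed maps track crafts and ghosts for removal by key.
; Ghosts store their GUID in CraftID, while real crafts get a map key without CraftID being set here.
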(fn `DestroyCraft`
  (params (Key :type "Guid Structure (by ref)"))
  (bind (_value _returnvalue) (`BlueprintMapLibrary.Map_Find` (`self.Crafts`) Key))
  (if _returnvalue
    (`Actor.K2_DestroyActor` _value)
    (`BlueprintMapLibrary.Map_Remove` (`self.Crafts`) (`local.Key`))))

(fn `DestroyGhostCraft`
  (params (Key :type "Guid Structure (by ref)"))
  (bind (_value _returnvalue) (`BlueprintMapLibrary.Map_Find` (`self.GhostCrafts`) Key))
  (if _returnvalue
    (`Actor.K2_DestroyActor` _value)
    (`BlueprintMapLibrary.Map_Remove` (`self.GhostCrafts`) (`local.Key`))))

(fn `GetCraftClass`
  (params (craft :type "/Game/Enums/E_Craft Enum" :default "NewEnumerator0"))
  (returns (Output_Get :type "Actor Class Reference"))
  (locals (Class :type "Actor Class Reference"))
  (switch `/Game/Enums/E_Craft` craft
    (:`NewEnumerator0`
      (set `local.Class` "/Game/BluePrints/Object/Craft/BP_Shelter.BP_Shelter_C"))
    (:`NewEnumerator1`
      (set `local.Class` "/Game/BluePrints/Object/Craft/BP_Fire.BP_Fire_C")))
  (return (`local.Class`)))

(fn `GetGhostCraft`
  (params (Selection :type "/Game/Enums/E_Craft Enum" :default "NewEnumerator0"))
  (returns (Output_Get :type "Actor Class Reference"))
  (locals (Class :type "Actor Class Reference"))
  (switch `/Game/Enums/E_Craft` Selection
    (:`NewEnumerator0`
      (set `local.Class` "/Game/BluePrints/Object/Craft/BP_GhostShelter.BP_GhostShelter_C"))
    (:`NewEnumerator1`
      (set `local.Class` "/Game/BluePrints/Object/Craft/BP_GhostFire.BP_GhostFire_C")))
  (return (`local.Class`)))

(fn `SpawnCraft`
  (params (craft :type "/Game/Enums/E_Craft Enum" :default "NewEnumerator0") (SpawnTransform :type "Transform Structure"))
  (bind _returnvalue (`|SpawnActorFromClass` (`self.GetCraftClass` craft) SpawnTransform "AlwaysSpawn" "OverrideRootScale" null null))
  (`BlueprintMapLibrary.Map_Add` (`self.Crafts`) (`KismetGuidLibrary.NewGuid`) (cast `/Game/BluePrints/Object/Craft/BP_BaseCraft` _returnvalue :!pure true)))

(fn `SpawnGhostCraft`
  (params (CraftClass :type "/Game/Enums/E_Craft Enum" :default "NewEnumerator0") (Tranform :type "Transform Structure"))
  (bind _returnvalue (`|SpawnActorFromClass` (`self.GetGhostCraft` CraftClass) Tranform "AlwaysSpawn" "OverrideRootScale" null null)) ; 모든 플레이어에게 해당 고스트 메쉬의 건축물을 생성한다
  (bind _asbp_base_craft (cast `/Game/BluePrints/Object/Craft/BP_BaseCraft` _returnvalue :!pure true))
  (bind _output_get (set `/Game/BluePrints/Object/Craft/BP_BaseCraft.CraftID` (`KismetGuidLibrary.NewGuid`) _asbp_base_craft))
  (`BlueprintMapLibrary.Map_Add` (`self.GhostCrafts`) _output_get _asbp_base_craft))