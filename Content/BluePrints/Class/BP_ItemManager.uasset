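; Item manager that spawns and destroys world pickups, trees and bushes, with a server event for creating new items.
; Initial spawns scatter fixed counts at random points inside the boxes of BP_SpawnItemSpot and BP_TreeSpawnActor actors.
; Each actor gets a new GUID and is stored in an item, tree or nature map for lookup and destruction by ID.
; An enum switch picks the item class, with Rope currently spawning BP_Meat.
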(event `Server_SpawnNewItem`
  (params (ItemType :type "/Game/Enums/E_ItemType Enum" :default "NewEnumerator0") (SpawnTransform :type "Transform Structure"))
  ;[1 1 1] Comment
  (`self.SpawnNewItem` ItemType SpawnTransform))

(event `SpawnItemFromGUID`
  ;[1 1 1] Comment
  (`self.SpawnItemList`))

(event `SpawnTreeFromGUID`
  ;[1 1 1] 나무 생성 / 삭제
  (`self.SpawnTreeList`))

(event `DestroyItemFromGUID`
  (params (ActorID :type "Guid Structure"))
  ;[1 1 1] Comment
  (`self.DestroyItem` ActorID))

(event `DestroyTreeFromGUID`
  (params (Key :type "Guid Structure (by ref)"))
  ;[1 1 1] 나무 생성 / 삭제
  (`self.DestroyTree` Key))

(fn `CheckCookingRecipe`)

(fn `DestroyItem`
  (params (ActorID :type "Guid Structure"))
  (bind (_value _returnvalue) (`BlueprintMapLibrary.Map_Find` (`self.ItemMap`) ActorID))
  ;[1 1 1] 코멘트
  (if _returnvalue
    (`Actor.K2_DestroyActor` _value)
    (bind _returnvalue_2 (`BlueprintMapLibrary.Map_Remove` (`self.ItemMap`) (`local.ActorID`)))
    (if _returnvalue_2
      (`KismetSystemLibrary.PrintString` "삭제 완료")
      (else
        (`KismetSystemLibrary.PrintString` "삭제 불가")))
    (else
      (`KismetSystemLibrary.PrintString` "액터 못찾음"))))

(fn `DestroyNature`
  (params (Key :type "Guid Structure (by ref)"))
  (bind (_value _returnvalue) (`BlueprintMapLibrary.Map_Find` (`self.NatureArray`) Key))
  ;[1 1 1] Comment
  (if _returnvalue
    (`Actor.K2_DestroyActor` _value)
    (`BlueprintMapLibrary.Map_Remove` (`self.NatureArray`) (`local.Key`))
    (`KismetSystemLibrary.PrintString` "덤불삭제")
    (else
      (`KismetSystemLibrary.PrintString` "액터 못찾음"))))

(fn `DestroyTree`
  (params (Key :type "Guid Structure (by ref)"))
  (bind (_value _returnvalue) (`BlueprintMapLibrary.Map_Find` (`self.TreeArray`) Key))
  (if _returnvalue
    (`Actor.K2_DestroyActor` _value)
    (`BlueprintMapLibrary.Map_Remove` (`self.TreeArray`) (`local.Key`))
    (else
      (`KismetSystemLibrary.PrintString` "나무 : ID에 해당되는 액터가 존재하지 않음"))))

(fn `GetItemActor`
  (params (ActorID :type "Guid Structure"))
  (returns (ItemActor :type "Actor Object Reference"))
  (bind (_value _returnvalue) (`BlueprintMapLibrary.Map_Find` (`self.ItemMap`) ActorID))
  ;[1 1 1] ID에 맞는 액터를 ItemList에서 빼서 가져온다.
  (if _returnvalue
    (return _value)
    (else
      (`KismetSystemLibrary.PrintString` "ID에 맞는 액터를 찾지 못함"))))

(fn `GetItemRandom Point`
  (params (Target :type "/Game/BluePrints/Object/Item/BP_SpawnItemSpot Object Reference"))
  (returns (RandomPoint :type "Vector Structure"))
  (bind (_returnvalue_x _returnvalue_y _returnvalue_z) (`KismetMathLibrary.BreakVector` (`Actor.K2_GetActorLocation` Target)))
  (bind (_returnvalue_x_2 _returnvalue_y_2) (`KismetMathLibrary.BreakVector` (`KismetMathLibrary.RandomPointInBoundingBox` (`Actor.K2_GetActorLocation` Target) (`BoxComponent.GetScaledBoxExtent` (`/Game/BluePrints/Object/Item/BP_SpawnItemSpot.Box` Target)))))
  ;[1 1 1] 스폰 포인트를 중심으로 Box Collider의 크기만큼의 지역에서 랜덤 포인트를 하나 지정해서 반환한다.
  (return (`KismetMathLibrary.MakeVector` _returnvalue_x_2 _returnvalue_y_2 _returnvalue_z)))

(fn `GetTreeRandomPoint`
  (params (TreeSpawnPoint :type "/Game/BluePrints/Object/Nature/BP_TreeSpawnActor Object Reference"))
  (returns (RandomPoint :type "Vector Structure"))
  (bind (_returnvalue_x _returnvalue_y _returnvalue_z) (`KismetMathLibrary.BreakVector` (`Actor.K2_GetActorLocation` TreeSpawnPoint)))
  (bind (_returnvalue_x_2 _returnvalue_y_2) (`KismetMathLibrary.BreakVector` (`KismetMathLibrary.RandomPointInBoundingBox` (`Actor.K2_GetActorLocation` TreeSpawnPoint) (`BoxComponent.GetScaledBoxExtent` (`/Game/BluePrints/Object/Nature/BP_TreeSpawnActor.Box` TreeSpawnPoint)))))
  ;[1 1 1] 스폰 포인트를 중심으로 Box Collider의 크기만큼의 지역에서 랜덤 포인트를 하나 지정해서 반환한다.
  (return (`KismetMathLibrary.MakeVector` _returnvalue_x_2 _returnvalue_y_2 _returnvalue_z)))

(fn `SpawnItemFromEnum`
  (params (ItemType :type "/Game/Enums/E_ItemType Enum" :default "NewEnumerator0") (SpawnTransform :type "Transform Structure"))
  (returns (ItemID :type "Guid Structure") (Item :type "/Game/BluePrints/Object/Item/BP_BaseItem Object Reference"))
  (locals (ItemClass :type "Actor Class Reference") (ID :type "Guid Structure") (ItemActor :type "/Game/BluePrints/Object/Item/BP_BaseItem Object Reference"))
  ;[1 1 1] 아이템을 생성한 뒤, 아이템에 대한 ID와 Actor값을 반환한다
  (switch `/Game/Enums/E_ItemType` ItemType
    (:`NewEnumerator0`
      (bind _returnvalue (`|SpawnActorFromClass` "/Game/BluePrints/Object/Item/BP_Branch.BP_Branch_C" (`local.SpawnTransform`) "Undefined" "OverrideRootScale" null null))
      (bind _itemid (`self.SetActorID` _returnvalue))
      (set `local.ID` _itemid)
      (set `local.ItemActor` _returnvalue))
    (:`NewEnumerator1`
      (bind _returnvalue_2 (`|SpawnActorFromClass` "/Game/BluePrints/Object/Item/BP_Wood.BP_Wood_C" (`local.SpawnTransform`) "Undefined" "OverrideRootScale" null null))
      (bind _itemid_2 (`self.SetActorID` _returnvalue_2))
      (set `local.ID` _itemid_2)
      (set `local.ItemActor` _returnvalue_2))
    (:`NewEnumerator5`
      (bind _returnvalue_3 (`|SpawnActorFromClass` "/Game/BluePrints/Object/Item/BP_Meat.BP_Meat_C" (`local.SpawnTransform`) "Undefined" "OverrideRootScale" null null))
      (bind _itemid_3 (`self.SetActorID` _returnvalue_3))
      (set `local.ID` _itemid_3)
      (set `local.ItemActor` _returnvalue_3))
    (:`NewEnumerator6`
      (bind _returnvalue_4 (`|SpawnActorFromClass` "/Game/BluePrints/Object/Item/BP_Blueberry.BP_Blueberry_C" (`local.SpawnTransform`) "Undefined" "OverrideRootScale" null null))
      (bind _itemid_4 (`self.SetActorID` _returnvalue_4))
      (set `local.ID` _itemid_4)
      (set `local.ItemActor` _returnvalue_4))
    (:`NewEnumerator7`
      (bind _returnvalue_5 (`|SpawnActorFromClass` "/Game/BluePrints/Object/Item/BP_Meat.BP_Meat_C" (`local.SpawnTransform`) "Undefined" "OverrideRootScale" null null))
      (bind _itemid_5 (`self.SetActorID` _returnvalue_5))
      (set `local.ID` _itemid_5)
      (set `local.ItemActor` _returnvalue_5))
    (:`NewEnumerator9`
      (bind _returnvalue_6 (`|SpawnActorFromClass` "/Game/BluePrints/Object/Item/BP_ZombieDummy.BP_ZombieDummy_C" (`local.SpawnTransform`) "Undefined" "OverrideRootScale" null null))
      (bind _itemid_6 (`self.SetActorID` _returnvalue_6))
      (set `local.ID` _itemid_6)
      (set `local.ItemActor` _returnvalue_6))
    (:`NewEnumerator10`
      (bind _returnvalue_7 (`|SpawnActorFromClass` "/Game/BluePrints/Object/Item/BP_Stone.BP_Stone_C" (`local.SpawnTransform`) "Undefined" "OverrideRootScale" null null))
      (bind _itemid_7 (`self.SetActorID` _returnvalue_7))
      (set `local.ID` _itemid_7)
      (set `local.ItemActor` _returnvalue_7))
    (:`NewEnumerator11`
      (bind _returnvalue_8 (`|SpawnActorFromClass` "/Game/BluePrints/Object/Item/BP_CookedMeat.BP_CookedMeat_C" (`local.SpawnTransform`) "Undefined" "OverrideRootScale" null null))
      (bind _itemid_8 (`self.SetActorID` _returnvalue_8))
      (set `local.ID` _itemid_8)
      (set `local.ItemActor` _returnvalue_8)))
  (return (`local.ID`) (`local.ItemActor`)))

(fn `SpawnItemList`
  (locals (Type :type "/Game/Enums/E_ItemType Enum"))
  ;[1 1 1] 초기화 : 정해진 아이템 리스트들을 토대로 아이템을 생성한다.
  (`KismetSystemLibrary.PrintString` "스폰 함수 진입")
  (bind _outactors (`GameplayStatics.GetAllActorsOfClass` "/Game/BluePrints/Object/Item/BP_SpawnItemSpot.BP_SpawnItemSpot_C"))
  (for _array_element _outactors
    (`self.SpawnItemReset` _array_element)))

(fn `SpawnItemReset`
  (params (SpawnPointActor :type "/Game/BluePrints/Object/Item/BP_SpawnItemSpot Object Reference"))
  (locals (enum :type "/Game/Enums/E_ItemType Enum") (Count :type Integer))
  (for _index (range 5)
    (switch `int` _index
      (:`0`
        (set `local.enum` "NewEnumerator0")
        (set `local.Count` 20))
      (:`1`
        (set `local.enum` "NewEnumerator6")
        (set `local.Count` 30))
      (:`2`
        (set `local.enum` "NewEnumerator10")
        (set `local.Count` 20))
      (:`3`
        (set `local.enum` "NewEnumerator5")
        (set `local.Count` 3)))
    (for _ (range (+ (`local.Count`) 1))
      (`self.SpawnNewItem` (`local.enum`) (`KismetMathLibrary.Conv_VectorToTransform` (`self.GetItemRandom Point` (`local.SpawnPointActor`)))))))

(fn `SpawnNature`
  (params (TreeSpawnPoint :type "/Game/BluePrints/Object/Nature/BP_TreeSpawnActor Object Reference"))
  ;[1 1 1] Comment
  (for _ (range 41)
    (bind _returnvalue (`|SpawnActorFromClass` "/Game/BluePrints/Object/Nature/BP_Bush01.BP_Bush01_C" (`KismetMathLibrary.Conv_VectorToTransform` (`self.GetTreeRandomPoint` (`local.TreeSpawnPoint`))) "Undefined" "OverrideRootScale" null null))
    (bind _output_get (set `/Game/BluePrints/Object/Nature/BP_BaseNature.NatureID` (`KismetGuidLibrary.NewGuid`) _returnvalue))
    (`BlueprintMapLibrary.Map_Add` (`self.NatureArray`) _output_get _returnvalue))
  (for _ (range 41)
    (bind _returnvalue_2 (`|SpawnActorFromClass` "/Game/BluePrints/Object/Nature/BP_Bush02.BP_Bush02_C" (`KismetMathLibrary.Conv_VectorToTransform` (`self.GetTreeRandomPoint` (`local.TreeSpawnPoint`))) "Undefined" "OverrideRootScale" null null))
    (bind _output_get_2 (set `/Game/BluePrints/Object/Nature/BP_BaseNature.NatureID` (`KismetGuidLibrary.NewGuid`) _returnvalue_2))
    (`BlueprintMapLibrary.Map_Add` (`self.NatureArray`) _output_get_2 _returnvalue_2)))

(fn `SpawnNatureList`
  ;[1 1 1] Comment
  (bind _outactors (`GameplayStatics.GetAllActorsOfClass` "/Game/BluePrints/Object/Nature/BP_TreeSpawnActor.BP_TreeSpawnActor_C"))
  (for _array_element _outactors
    (`self.SpawnNature` _array_element)))

(fn `SpawnNewItem`
  (params (ItemType :type "/Game/Enums/E_ItemType Enum" :default "NewEnumerator0") (SpawnTransform :type "Transform Structure"))
  (locals (`DS Item` :type " Structure"))
  (bind (_itemid _item) (`self.SpawnItemFromEnum` ItemType SpawnTransform))
  ;[1 1 1] ItemType에 맞는 액터를 지정 위치에 생성
  (`BlueprintMapLibrary.Map_Add` (`self.ItemMap`) _itemid _item)
  (`KismetSystemLibrary.PrintString` "아이템 추가 완료"))

(fn `SpawnTreeList`
  (bind _outactors (`GameplayStatics.GetAllActorsOfClass` "/Game/BluePrints/Object/Nature/BP_TreeSpawnActor.BP_TreeSpawnActor_C"))
  (for _array_element _outactors
    (`self.SpawnTrees` _array_element)))

(fn `SpawnTrees`
  (params (SpawnPoint :type "/Game/BluePrints/Object/Nature/BP_TreeSpawnActor Object Reference"))
  (locals (MaxTreeCount :type Integer :default 50))
  ;[1 1 1] 코멘트
  (for _ (range (`local.MaxTreeCount`))
    (bind _returnvalue (`|SpawnActorFromClass` "/Game/BluePrints/Object/Nature/BP_Tree01.BP_Tree01_C" (`KismetMathLibrary.Conv_VectorToTransform` (`self.GetTreeRandomPoint` (`local.SpawnPoint`))) "Undefined" "OverrideRootScale" null null))
    (bind _output_get (set `/Game/BluePrints/Object/Nature/BP_BaseTree.TreeID` (`KismetGuidLibrary.NewGuid`) _returnvalue))
    (`BlueprintMapLibrary.Map_Add` (`self.TreeArray`) _output_get _returnvalue))
  (for _ (range (`local.MaxTreeCount`))
    (bind _returnvalue_2 (`|SpawnActorFromClass` "/Game/BluePrints/Object/Nature/BP_Tree02.BP_Tree02_C" (`KismetMathLibrary.Conv_VectorToTransform` (`self.GetTreeRandomPoint` (`local.SpawnPoint`))) "Undefined" "OverrideRootScale" null null))
    (bind _output_get_2 (set `/Game/BluePrints/Object/Nature/BP_BaseTree.TreeID` (`KismetGuidLibrary.NewGuid`) _returnvalue_2))
    (`BlueprintMapLibrary.Map_Add` (`self.TreeArray`) _output_get_2 _returnvalue_2)))