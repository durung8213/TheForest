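; BP_PlayerStatus is a player character component that manages replicated health, hunger, thirst and dash energy, with OnRep functions updating the HUD.
; An authority-started looping timer decays hunger and thirst; low hunger lowers the energy cap and low thirst damages health.
; Dash requests go through server and multicast events to change walk speed, with looping timers draining energy, stopping the dash when empty, and recovering it.
; Increase functions restore each stat with clamping.
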(event `Owner_GetDamaged`
  (params (DamegePoint :type "Float (double-precision)"))
  ;[1 1 1] HP 감소
  (`self.Server_GetDamaged` DamegePoint))

(event `self.ReceiveBeginPlay`
  ;[1 1 1] 시작 : 계속해서 생존 수치 감소
  (bind _asbp_player_character (cast `/Game/Character/BP_PlayerCharacter` (`self.GetOwner`)))
  (set `self.OwnerPlayer` _asbp_player_character)
  (if (`Actor.HasAuthority` _asbp_player_character)
    (bind _returnvalue (`KismetSystemLibrary.K2_SetTimerDelegate` (delegate `Owner_DecreaseStat`) 5.0 true)) ; 일정 시간 마다 허기 / 목마름 수치가 감소하도록
    (set `self.StatDecTH` _returnvalue)))

(event `Server_GetDamaged`
  (params (DamegePoint :type "Float (double-precision)"))
  ;[1 1 1] HP 감소
  (`self.GetDamaged` DamegePoint))

(event `Owner_DecreaseStat`
  ;[1 1 1] 시작 : 계속해서 생존 수치 감소
  (`self.Server_DecreaseStat`))

(event `Server_DecreaseStat`
  ;[1 1 1] 시작 : 계속해서 생존 수치 감소
  (`self.DecreaseStat`))

(event `Owner_StartDash`
  ;[1 1 1] 대쉬 스타트
  (`self.Server_StartDash`))

(event `Owner_StopDash`
  ;[1 1 1] 대쉬 스탑
  (`self.Server_StopDash`))

(event `Server_StartDash`
  ;[1 1 1] 대쉬 스타트
  (`self.Multi_StartDash`))

(event `Server_StopDash`
  ;[1 1 1] 대쉬 스탑
  (`self.Multi_StopDash`))

(event `Multi_StopDash`
  ;[1 1 1] 대쉬 스탑
  (`self.StopDash`))

(event `Multi_StartDash`
  ;[1 1 1] 대쉬 스타트
  (`self.StartDash`))

(fn `DecreaseEnergy`
  ;[1 1 1] StartDash 타이머에서 반복되는 에너지 감소 함수
  (set `self.CurrentEnergy` (`KismetMathLibrary.FClamp` (- (`self.CurrentEnergy`) (`self.DashCost`)) 0.0 (`self.MaxEnergy`)))
  (if (<= (`self.CurrentEnergy`) 0.0)
    (`self.Owner_StopDash`)))

(fn `DecreaseStat`
  (locals (E_MaxPoint :type "Float (double-precision)") (DecreasePoint :type "Float (double-precision)" :default 0.02))
  ;[1 1 1] 코멘트
  (if (`Actor.HasAuthority` (`GameplayStatics.GetPlayerController` 0))
    (set `self.Hungry` (`KismetMathLibrary.FClamp` (- (`self.Hungry`) (`local.DecreasePoint`)) 0.01))
    (set `self.Thirsty` (`KismetMathLibrary.FClamp` (- (`self.Thirsty`) (`local.DecreasePoint`)) 0.01))
    (if (< (`self.Hungry`) 0.5)
      (set `self.MaxEnergy` 0.4)
      (else
        (set `self.MaxEnergy` 1.0)))
    (if (< (`self.Thirsty`) 0.5)
      (`self.GetDamaged` 0.01) ; 조금씩 체력이 줄어든다.
    )))

(fn `GetDamaged`
  (params (DamegePoint :type "Float (double-precision)"))
  ;[1 1 1] NPC 에게 맞을 경우
  (set `self.Health` (- (`self.Health`) DamegePoint)))

(fn `GetPlayerHUD`
  (returns (`AsBP World HUD` :type "/Game/BluePrints/HUD/BP_WorldHUD Object Reference"))
  ;[1 1 1] 캐릭터의 HUD 가져오기
  (bind _asbp_player_character (cast `/Game/Character/BP_PlayerCharacter` (`self.GetOwner`)))
  (bind _asbp_world_pc (cast `/Game/BluePrints/PlayerController/BP_WorldPC` (`Pawn.GetController` _asbp_player_character)))
  (bind _asbp_world_hud (cast `/Game/BluePrints/HUD/BP_WorldHUD` (`PlayerController.GetHUD` _asbp_world_pc)))
  (return _asbp_world_hud))

(fn `IncreaseEnergy`
  (params (value :type "Float (double-precision)"))
  (set `self.CurrentEnergy` (`KismetMathLibrary.FClamp` (+ value (`self.CurrentEnergy`)) 0.0 (`self.MaxEnergy`))))

(fn `IncreaseHealth`
  (params (value :type "Float (double-precision)"))
  (set `self.Health` (`KismetMathLibrary.FClamp` (+ value (`self.Health`)))))

(fn `IncreaseHungry`
  (params (value :type "Float (double-precision)"))
  (set `self.Hungry` (`KismetMathLibrary.FClamp` (+ value (`self.Hungry`)))))

(fn `IncreaseThirsty`
  (params (value :type "Float (double-precision)"))
  (set `self.Thirsty` (`KismetMathLibrary.FClamp` (+ value (`self.Thirsty`)))))

(fn `OnRep_Energy`
  (bind _asbp_world_hud (`self.GetPlayerHUD`))
  (`/Engine/EditorBlueprintResources/StandardMacros.IsValid` _asbp_world_hud
    (:`Is Valid`
      (`/Game/BluePrints/HUD/BP_WorldHUD.UpdateEnergyUI` _asbp_world_hud (`self.CurrentEnergy`)))))

(fn `OnRep_Health`
  (bind _asbp_world_hud (`self.GetPlayerHUD`))
  (`/Engine/EditorBlueprintResources/StandardMacros.IsValid` _asbp_world_hud
    (:`Is Valid`
      (`/Game/BluePrints/HUD/BP_WorldHUD.UpdateHealthUI` _asbp_world_hud (`self.Health`)))))

(fn `OnRep_Hungry`
  (bind _asbp_world_hud (`self.GetPlayerHUD`))
  (`/Engine/EditorBlueprintResources/StandardMacros.IsValid` _asbp_world_hud
    (:`Is Valid`
      (`/Game/BluePrints/HUD/BP_WorldHUD.UpdateHungerUI` _asbp_world_hud (`self.Hungry`)))))

(fn `OnRep_Thirsty`
  (bind _asbp_world_hud (`self.GetPlayerHUD`))
  (`/Engine/EditorBlueprintResources/StandardMacros.IsValid` _asbp_world_hud
    (:`Is Valid`
      (`/Game/BluePrints/HUD/BP_WorldHUD.UpdateThirstUI` _asbp_world_hud (`self.Thirsty`)))))

(fn `RecoveryEnergy`
  ;[1 1 1] 코멘트
  (if (<= (`self.CurrentEnergy`) (`self.MaxEnergy`))
    (set `self.CurrentEnergy` (`KismetMathLibrary.FClamp` (+ (`self.CurrentEnergy`) (`self.DashCost`)) 0.0 (`self.MaxEnergy`)))))

(fn `StartDash`
  (locals (DashSpeed :type "Float (double-precision)" :default 800.0))
  ;[1 1 1] 대쉬 시작
  (if (not (`self.IsDashing`))
    (`KismetSystemLibrary.K2_ClearAndInvalidateTimerHandle` (`self.RecoverEnergyTH`))
    (set `self.IsDashing` true)
    (bind _asbp_player_character (cast `/Game/Character/BP_PlayerCharacter` (`self.GetOwner`)))
    (set `CharacterMovementComponent.MaxWalkSpeed` (`local.DashSpeed`) (`Character.CharacterMovement` _asbp_player_character))
    (if (`KismetSystemLibrary.K2_IsTimerActiveHandle` (`self.DashEnergyTH`))
      (`KismetSystemLibrary.K2_ClearAndInvalidateTimerHandle` (`self.DashEnergyTH`)))
    (bind _returnvalue (`KismetSystemLibrary.K2_SetTimer` null "DecreaseEnergy" 0.01 true))
    (set `self.DashEnergyTH` _returnvalue)))

(fn `StopDash`
  (locals (OriginWalkSpeed :type "Float (double-precision)" :default 330.0))
  ;[1 1 1] 대쉬 : 만약 대쉬 게이지가 0이 되면 대쉬가 멈추고, 자동으로 대쉬 게이지가 증가하도록 설정
  (if (`self.IsDashing`)
    (set `self.IsDashing` false)
    (set `CharacterMovementComponent.MaxWalkSpeed` (`local.OriginWalkSpeed`) (`Character.CharacterMovement` (`self.OwnerPlayer`)))
    (`KismetSystemLibrary.K2_ClearAndInvalidateTimerHandle` (`self.DashEnergyTH`)) ; 대쉬를 실행하는 타이머를 멈춤
    (if (`KismetSystemLibrary.K2_IsTimerActiveHandle` (`self.RecoverEnergyTH`))
      (`KismetSystemLibrary.K2_ClearAndInvalidateTimerHandle` (`self.RecoverEnergyTH`)))
    (bind _returnvalue (`KismetSystemLibrary.K2_SetTimer` null "RecoveryEnergy" 0.01 true))
    (set `self.RecoverEnergyTH` _returnvalue)))