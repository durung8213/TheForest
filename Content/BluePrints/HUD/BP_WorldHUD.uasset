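; BP_WorldHUD is the HUD for a survival game, creating quick slot and player status widgets at BeginPlay.
; Show/hide functions manage pickup, inventory, crafting, build preview, campfire cooking and option widgets, with inventory, craft book and options also toggling cursor and input mode.
; Inventory, quick slot and craft mode refresh by recreating their widgets, while health, hunger, thirst and energy updates set progress bars directly.
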(event `self.ReceiveBeginPlay`
  ;[1 1 1] 코멘트
  (bind _returnvalue (`|CreateWidget` "/Game/UIWidget/Player/WBP_QuickSlot.WBP_QuickSlot_C" (`GameplayStatics.GetPlayerController` 0)))
  (bind _output_get (set `self.QuickSlotUI` _returnvalue))
  (`UserWidget.AddToViewport` _output_get 0)
  (bind _returnvalue_2 (`|CreateWidget` "/Game/UIWidget/Player/WBP_PlayerStatus.WBP_PlayerStatus_C" (`GameplayStatics.GetPlayerController` 0)))
  (bind _output_get_2 (set `self.PlayerStat` _returnvalue_2))
  (`UserWidget.AddToViewport` _output_get_2 0)
  (`WidgetBlueprintLibrary.SetInputMode_GameOnly` (`GameplayStatics.GetPlayerController` 0))
  (set `PlayerController.bShowMouseCursor` false (`GameplayStatics.GetPlayerController` 0)))

(event `UpdateInventory`
  ;[1 1 1] Inventory / Quick Slot
  (`self.UpdateInventoryUI`))

(event `UpdateToolSlot`
  ;[1 1 1] Inventory / Quick Slot
  (`self.UpdateToolsUI`))

(fn `CloseInventory`
  (bind _returnvalue (`GameplayStatics.GetPlayerController` 0))
  (`WidgetBlueprintLibrary.SetInputMode_GameOnly` _returnvalue)
  (set `PlayerController.bShowMouseCursor` false _returnvalue)
  (`Widget.RemoveFromParent` (`self.InventoryUI`)))

(fn `HideCookingUI`
  (bind _campfireui (`self.CampFireUI`)
    (:`then`
      (`Widget.RemoveFromParent` _campfireui))
    (:`else`)))

(fn `HideCraftBookUI`
  (bind _returnvalue (`GameplayStatics.GetPlayerController` 0))
  ;[1 1 1] CraftBook UI 숨기기
  (`WidgetBlueprintLibrary.SetInputMode_GameOnly` _returnvalue)
  (set `PlayerController.bShowMouseCursor` false _returnvalue)
  (bind _craftbookui (`self.CraftBookUI`)
    (:`then`
      (`Widget.RemoveFromParent` _craftbookui))
    (:`else`)))

(fn `HideCraftModeUI`
  (bind _craftmodeui (`self.CraftModeUI`)
    (:`then`
      (`Widget.RemoveFromParent` _craftmodeui))
    (:`else`)))

(fn `HideOptionUI`
  (bind _asbp_world_pc (cast `/Game/BluePrints/PlayerController/BP_WorldPC` (`self.GetOwningPlayerController`)))
  (`WidgetBlueprintLibrary.SetInputMode_GameOnly` _asbp_world_pc)
  (set `PlayerController.bShowMouseCursor` false _asbp_world_pc)
  (bind _optionui (`self.OptionUI`)
    (:`then`
      (`Widget.RemoveFromParent` _optionui))
    (:`else`)))

(fn `HidePickUpItem`
  (bind _pickupicon (`self.PickUpIcon`)
    (:`then`
      (`Widget.RemoveFromParent` _pickupicon))
    (:`else`)))

(fn `HidePreviewIcon`
  (bind _previewbuildingicon (`self.PreviewBuildingIcon`)
    (:`then`
      (`Widget.RemoveFromParent` _previewbuildingicon))
    (:`else`)))

(fn `OpenInventory`
  (bind _returnvalue (`GameplayStatics.GetPlayerController` 0))
  ;[1 1 1] Inventory UI Open
  (bind _returnvalue_2 (`|CreateWidget` "/Game/UIWidget/Player/WBP_Inventory.WBP_Inventory_C" _returnvalue))
  (bind _output_get (set `self.InventoryUI` _returnvalue_2))
  (`UserWidget.AddToViewport` _output_get 0)
  (set `PlayerController.bShowMouseCursor` true _returnvalue)
  (`WidgetBlueprintLibrary.SetInputMode_GameAndUIEx` _returnvalue null))

(fn `Show Pick Up Item`
  ;[1 1 1] 아이템 획득 가능 UI 표시
  (if (`KismetSystemLibrary.IsValid` (`self.PickUpIcon`))
    (if (not (`Widget.IsInViewport` (`self.PickUpIcon`)))
      (bind _returnvalue (`|CreateWidget` "/Game/UIWidget/WBP_PickUpItemUI.WBP_PickUpItemUI_C" (`GameplayStatics.GetPlayerController` 0) :!label _label))
      (bind _output_get (set `self.PickUpIcon` _returnvalue))
      (`UserWidget.AddToViewport` _output_get 0))
    (else
      (goto _label))))

(fn `ShowCookingUI`
  (bind _returnvalue (`|CreateWidget` "/Game/UIWidget/Craft/WBP_CampFire.WBP_CampFire_C"))
  (bind _output_get (set `self.CampFireUI` _returnvalue))
  (`UserWidget.AddToViewport` _output_get 0))

(fn `ShowCraftBookUI`
  (bind _returnvalue (`GameplayStatics.GetPlayerController` 0))
  ;[1 1 1] Craft UI Open
  (bind _returnvalue_2 (`|CreateWidget` "/Game/UIWidget/Craft/WBP_CraftPage.WBP_CraftPage_C" _returnvalue))
  (bind _output_get (set `self.CraftBookUI` _returnvalue_2))
  (`UserWidget.AddToViewport` _output_get 0)
  (set `PlayerController.bShowMouseCursor` true _returnvalue)
  (`WidgetBlueprintLibrary.SetInputMode_GameAndUIEx` _returnvalue (`self.CraftBookUI`)))

(fn `ShowCraftModeUI`
  (params (CurrentCraft :type "/Game/BluePrints/Object/Craft/BP_BaseCraft Object Reference"))
  ;[1 1 1] Comment
  (bind _returnvalue (`|CreateWidget` "/Game/UIWidget/Craft/WBP_CraftMode.WBP_CraftMode_C" (`GameplayStatics.GetPlayerController` 0)))
  (set `/Game/UIWidget/Craft/WBP_CraftMode.CurrentCraft` CurrentCraft _returnvalue)
  (bind _output_get (set `self.CraftModeUI` _returnvalue))
  (`UserWidget.AddToViewport` _output_get 0)
  (`KismetSystemLibrary.PrintString` "add viewport"))

(fn `ShowOptionUI`
  (bind _returnvalue (`|CreateWidget` "/Game/UIWidget/WBP_Option.WBP_Option_C"))
  (set `self.OptionUI` _returnvalue)
  (bind _asbp_world_pc (cast `/Game/BluePrints/PlayerController/BP_WorldPC` (`self.GetOwningPlayerController`)))
  (`WidgetBlueprintLibrary.SetInputMode_GameAndUIEx` _asbp_world_pc null)
  (set `PlayerController.bShowMouseCursor` true _asbp_world_pc)
  (`UserWidget.AddToViewport` (`self.OptionUI`) 0))

(fn `ShowPreviewIcon`
  (bind _returnvalue (`|CreateWidget` "/Game/UIWidget/Player/WBP_PreviewBuildingIcon.WBP_PreviewBuildingIcon_C" (`GameplayStatics.GetPlayerController` 0)))
  (bind _output_get (set `self.PreviewBuildingIcon` _returnvalue))
  (`UserWidget.AddToViewport` _output_get 0))

(fn `UpdateCraftModeUI`
  (params (CraftBuilding :type "/Game/BluePrints/Object/Craft/BP_BaseCraft Object Reference"))
  (`KismetSystemLibrary.PrintString` "업데이트UI")
  (bind _craftmodeui (`self.CraftModeUI`)
    (:`then`
      (if (`Widget.IsVisible` _craftmodeui)
        (`self.HideCraftModeUI`)
        (`self.ShowCraftModeUI` CraftBuilding)))
    (:`else`)))

(fn `UpdateEnergyUI`
  (params (InPercent :type "Float (double-precision)"))
  (`ProgressBar.SetPercent` (`/Game/UIWidget/Player/WBP_PlayerStatus.EnergyBar` (`self.PlayerStat`)) InPercent))

(fn `UpdateHealthUI`
  (params (InPercent :type "Float (double-precision)"))
  (`ProgressBar.SetPercent` (`/Game/UIWidget/Player/WBP_PlayerStatus.HPBar` (`self.PlayerStat`)) InPercent)
  (`KismetSystemLibrary.PrintString` (`KismetStringLibrary.Conv_DoubleToString` InPercent))
  (`KismetSystemLibrary.PrintString` "UI"))

(fn `UpdateHungerUI`
  (params (InPercent :type "Float (double-precision)"))
  (`KismetSystemLibrary.PrintString` (`KismetStringLibrary.Conv_DoubleToString` InPercent))
  (`ProgressBar.SetPercent` (`/Game/UIWidget/Player/WBP_PlayerStatus.HungerBar` (`self.PlayerStat`)) InPercent))

(fn `UpdateInventoryUI`
  ;[1 1 1] 인벤토리 상태가 갱신될 때, 인벤토리 UI가 활성화 되어있다면 다시 인벤토리 UI를 그리도록 한다.
  (bind _inventoryui (`self.InventoryUI`) ; 현재 인벤토리 UI가 표시되어 있는지 아닌지 확인.
    (:`then`
      (if (`Widget.IsVisible` _inventoryui)
        (`self.CloseInventory`) ; 인벤토리를 닫았다가 다시 열기
        (`self.OpenInventory`)))
    (:`else`)))

(fn `UpdateThirstUI`
  (params (InPercent :type "Float (double-precision)"))
  (`KismetSystemLibrary.PrintString` "목마름 수치 :")
  (`KismetSystemLibrary.PrintString` (`KismetStringLibrary.Conv_DoubleToString` InPercent))
  (`ProgressBar.SetPercent` (`/Game/UIWidget/Player/WBP_PlayerStatus.ThirstBar` (`self.PlayerStat`)) InPercent))

(fn `UpdateToolsUI`
  ;[1 1 1] QuickSlot Update
  (`Widget.RemoveFromParent` (`self.QuickSlotUI`))
  (bind _returnvalue (`|CreateWidget` "/Game/UIWidget/Player/WBP_QuickSlot.WBP_QuickSlot_C" (`GameplayStatics.GetPlayerController` 0)))
  (bind _output_get (set `self.QuickSlotUI` _returnvalue))
  (`UserWidget.AddToViewport` _output_get 0))

(fn `UserConstructionScript`
  (`parent.UserConstructionScript`))