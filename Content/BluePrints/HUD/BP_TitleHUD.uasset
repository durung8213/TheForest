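; BP_TitleHUD is the HUD Blueprint that brings up the title screen.
; On BeginPlay it creates the WBP_Title widget for player controller 0 and adds it to the viewport.
; It then switches that controller to UI-only input focused on the widget, with an unlocked, visible mouse cursor, and prints the current GameMode's name as debug output.
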(event `self.ReceiveBeginPlay`
  (bind _returnvalue (`|CreateWidget` "/Game/UIWidget/WBP_Title.WBP_Title_C" (`GameplayStatics.GetPlayerController` 0)))
  (`UserWidget.AddToViewport` _returnvalue 0)
  (`WidgetBlueprintLibrary.SetInputMode_UIOnlyEx` (`GameplayStatics.GetPlayerController` 0) _returnvalue)
  (set `PlayerController.bShowMouseCursor` true (`GameplayStatics.GetPlayerController` 0))
  (`KismetSystemLibrary.PrintString` (`KismetSystemLibrary.GetDisplayName` (`GameplayStatics.GetGameMode`))))

(fn `UserConstructionScript`
  (`parent.UserConstructionScript`))