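; BP_AIZombieController is the zombie AI controller that starts the zombie's blackboard and behavior tree.
; On possess, RunAI loads the blackboard asset and stores the pawn's current location as the home position key.
; It then runs the behavior tree and prints whether the start succeeded or failed.
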(event `self.ReceivePossess`
  (params (PossessedPawn :type "Pawn Object Reference"))
  (`self.RunAI`))

(event `RunAI`
  (bind (_blackboardcomponent _returnvalue) (`self.UseBlackboard` (`self.BlackBoardAsset`))) ; 블랙보드를 설정
  (if _returnvalue
    (set `self.BBComponent` _blackboardcomponent) ; 블랙보드 안에 있는 컴포넌트 설정
    (`BlackboardComponent.SetValueAsVector` (`self.BBComponent`) (`self.KeyHomePos`) (`self.K2_GetActorLocation` (`self.K2_GetPawn`))) ; 블랙보드의 키 값을 정한다. 블랙보드가 가지고 있는 함수를 통해서 설정.
    (bind _returnvalue_2 (`self.RunBehaviorTree` (`self.BTAsset`)))
    (if _returnvalue_2
      (`KismetSystemLibrary.PrintString` "AI Run Seccess")
      (else
        (`KismetSystemLibrary.PrintString` "AI Run Fail")))))

(fn `UserConstructionScript`)