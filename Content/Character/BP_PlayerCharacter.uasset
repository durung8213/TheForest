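; Player character Blueprint for a multiplayer survival-crafting game, handling axe use, zombie damage, gathering and building.
; Owner events forward to Server RPCs, with equip, tool montage and zombie damage multicast to clients.
; Crafting, leaf pickup and item spawning stay on the server, using the inventory component and GameMode's craft and item managers.
; The equipped axe attaches to a mesh socket and flags the AnimBP, while the replicated name updates its label after a delay.
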(event `Owner_UnEquipTool`
  ;[1 1 1] 장비 해제
  (`self.Server_UnEquipTool`))

(event `Owner_EquipTool`
  (params (Selection :type "/Game/Enums/E_Tool Enum" :default "NewEnumerator0"))
  ;[1 1 1] 장비 장착
  (`self.Server_EquipTool` Selection))

(event `Server_UnEquipTool`
  ;[1 1 1] 장비 해제
  (`self.Multi_UnEquipTool`)
  (set `self.IsAxeEquip` false))

(event `Server_EquipTool`
  (params (Selection :type "/Game/Enums/E_Tool Enum" :default "NewEnumerator0"))
  ;[1 1 1] 장비 장착
  (`self.Multi_EquipTool` Selection)
  (set `self.IsAxeEquip` true))

(event `Multi_UnEquipTool`
  ;[1 1 1] 장비 해제
  (bind _toolactor (`self.ToolActor`)
    (:`then`
      (`self.UnEquipToolItem` _toolactor))
    (:`else`)))

(event `Multi_EquipTool`
  (params (Selection :type "/Game/Enums/E_Tool Enum" :default "NewEnumerator0"))
  ;[1 1 1] 장비 장착
  (`self.EquipToolItem` Selection))

(event `Owner_ToolAction`
  (params (CurrentTool :type "/Game/Enums/E_Tool Enum" :default "NewEnumerator0"))
  ;[1 1 1] 왼쪽 마우스 입력 : 도구 사용
  (`self.Server_ToolAction` CurrentTool))

(event `Owner_CraftBuilding`
  (params (craft :type "/Game/BluePrints/Object/Craft/BP_BaseCraft Object Reference"))
  ;[1 1 1] Craft Building : 재료 추가하기
  (`self.Server_CraftBuilding` craft))

(event `Owner_AttackZombie`
  (params (zombie :type "/Game/Character/BP_AIZombie Object Reference") (attackPoint :type "Float (double-precision)"))
  ;[1 1 1] 도끼 공격 : 좀비
  (`self.Server_AttackZombie` zombie attackPoint))

(event `Server_CraftBuilding`
  (params (craft :type "/Game/BluePrints/Object/Craft/BP_BaseCraft Object Reference"))
  ;[1 1 1] Craft Building : 재료 추가하기
  (`self.CraftBuilding` craft))

(event `Server_ToolAction`
  (params (CurrentTool :type "/Game/Enums/E_Tool Enum" :default "NewEnumerator0"))
  ;[1 1 1] 왼쪽 마우스 입력 : 도구 사용
  (`self.Multi_ToolAction` CurrentTool))

(event `Server_AttackZombie`
  (params (zombie :type "/Game/Character/BP_AIZombie Object Reference") (attackPoint :type "Float (double-precision)"))
  ;[1 1 1] 도끼 공격 : 좀비
  (`self.Multi_AttackZombie` zombie attackPoint))

(event `Multi_ToolAction`
  (params (CurrentTool :type "/Game/Enums/E_Tool Enum" :default "NewEnumerator0"))
  ;[1 1 1] 왼쪽 마우스 입력 : 도구 사용
  (`self.ToolAction` CurrentTool))

(event `Multi_AttackZombie`
  (params (zombie :type "/Game/Character/BP_AIZombie Object Reference") (attackPoint :type "Float (double-precision)"))
  ;[1 1 1] 도끼 공격 : 좀비
  (`self.AttackZombie` zombie attackPoint))

(event `Owenr_AddLeafToInven`
  (params (Key :type "Guid Structure (by ref)"))
  ;[1 1 1] 도끼로 나뭇잎 베기
  (`self.Server_AddLeafToInven` Key))

(event `Server_RequestSpawnItem`
  (params (ItemType :type "/Game/Enums/E_ItemType Enum" :default "NewEnumerator0") (SpawnTransform :type "Transform Structure"))
  (`self.RequestSpawnItem` ItemType SpawnTransform))

(event `Server_AddLeafToInven`
  (params (Key :type "Guid Structure (by ref)"))
  ;[1 1 1] 도끼로 나뭇잎 베기
  (`self.AddLeafToInven` Key))

(fn `AddLeafToInven`
  (params (Key :type "Guid Structure (by ref)"))
  ;[1 1 1] 나뭇잎 아이템 추가
  (bind _returnvalue (`|GetDataTableRow` "/Game/DataTable/DT_ItemList.DT_ItemList" "5")
    (:`then`
      (`/Game/BluePrints/Class/BP_PlayerInventory.Add Item to Inventory` (`self.BP_PlayerInventory`) _returnvalue)
      (bind _asbp_world_gm (cast `/Game/BluePrints/GameMode/BP_WorldGM` (`GameplayStatics.GetGameMode`)))
      (`/Game/BluePrints/Class/BP_ItemManager.DestroyNature` (`/Game/BluePrints/GameMode/BP_WorldGM.BP_ItemManager` _asbp_world_gm) (`local.Key`)))))

(fn `AttackZombie`
  (params (zombie :type "/Game/Character/BP_AIZombie Object Reference") (attackPoint :type "Float (double-precision)"))
  (bind _output_get (set `/Game/Character/BP_AIZombie.ZombieHP` (`KismetMathLibrary.FClamp` (- (`/Game/Character/BP_AIZombie.ZombieHP` zombie) attackPoint) 0.0 100.0) (`local.zombie`)))
  (`KismetSystemLibrary.PrintString` (`KismetStringLibrary.Conv_DoubleToString` _output_get)))

(fn `CraftBuilding`
  (params (craft :type "/Game/BluePrints/Object/Craft/BP_BaseCraft Object Reference"))
  (bind _craft (`local.craft`))
  (bind _craft_2 (`local.craft`))
  (bind _craft_3 (`local.craft`))
  ;[1 1 1] Comment
  (`KismetSystemLibrary.PrintString` "Craftin")
  (set `/Game/BluePrints/Object/Craft/BP_BaseCraft.IsProcessing` true _craft)
  (bind (_returnvalue _itemtype) (`/Game/BluePrints/Class/BP_PlayerInventory.CheckItemFromEnum` (`self.BP_PlayerInventory`) _craft)) ; 해당 타입의 아이템이 인벤토리에 있는지 확인
  (if _returnvalue
    (`/Game/BluePrints/Object/Craft/BP_BaseCraft.PlusCount` (`local.craft`) _itemtype) ; 현재 객체의 배열에 Count를 증가시킨다.
    (`KismetSystemLibrary.PrintString` "객체 수 증가")
    (set `/Game/BluePrints/Object/Craft/BP_BaseCraft.IsProcessing` false _craft_2)
    (`/Game/BluePrints/Class/BP_PlayerInventory.UseItemToDecrease` (`self.BP_PlayerInventory`) _itemtype) ; 인벤토리의 아이템을 삭제시킨다
    (if (`/Game/BluePrints/Object/Craft/BP_BaseCraft.CheckItemArray` (`local.craft`))
      (bind _asbp_world_gm (cast `/Game/BluePrints/GameMode/BP_WorldGM` (`GameplayStatics.GetGameMode`)))
      (`KismetSystemLibrary.PrintString` "삭제시작")
      (bind _bp_craftmanager (`/Game/BluePrints/GameMode/BP_WorldGM.BP_CraftManager` _asbp_world_gm))
      (`/Game/BluePrints/Class/BP_CraftManager.SpawnCraft` _bp_craftmanager (`/Game/BluePrints/Object/Craft/BP_BaseCraft.CraftType` _craft_3) (`self.GetTransform` _craft_3))
      (`/Game/BluePrints/Class/BP_CraftManager.DestroyGhostCraft` _bp_craftmanager (`/Game/BluePrints/Object/Craft/BP_BaseCraft.CraftID` _craft_3)))
    (else
      (set `/Game/BluePrints/Object/Craft/BP_BaseCraft.IsProcessing` false _craft_2))))

(fn `Dash`)

(fn `EquipToolItem`
  (params (Selection :type "/Game/Enums/E_Tool Enum" :default "NewEnumerator0"))
  ;[1 1 1] 플레이어 소켓에 도구 붙이기
  (switch `/Game/Enums/E_Tool` Selection ; 도구에 따라 스폰되는 액터가 다름
    (:`NewEnumerator0`
      (bind _returnvalue (`|SpawnActorFromClass` "/Game/BluePrints/Object/Tool/BP_Axe.BP_Axe_C" (`self.GetTransform` self) "AdjustIfPossibleButAlwaysSpawn" "OverrideRootScale" null null))
      (bind _output_get (set `self.ToolActor` _returnvalue))
      (`self.SetOwner` _output_get self)
      (`self.K2_AttachToComponent` _output_get (`self.Mesh`) "Axe" "SnapToTarget" "SnapToTarget" "KeepRelative" true)
      (bind _asabp_player (cast `/Game/Character/ABP/ABP_Player` (`SkeletalMeshComponent.GetAnimInstance` (`self.Mesh`))))
      (set `/Game/Character/ABP/ABP_Player.IsHoldingAxe` true _asabp_player))))

(fn `IsPlayer`
  (returns (IsPlayer :type Boolean))
  (return true))

(fn `OnRep_PlayerName`
  (bind _returnvalue (`KismetSystemLibrary.K2_SetTimer` null "ShowPlayerName" 0.5))
  (set `self.NameTH` _returnvalue))

(fn `RequestSpawnItem`
  (params (ItemType :type "/Game/Enums/E_ItemType Enum" :default "NewEnumerator0") (SpawnTransform :type "Transform Structure"))
  (bind _asbp_world_gm (cast `/Game/BluePrints/GameMode/BP_WorldGM` (`GameplayStatics.GetGameMode`)))
  (`/Game/BluePrints/Class/BP_ItemManager.SpawnNewItem` (`/Game/BluePrints/GameMode/BP_WorldGM.BP_ItemManager` _asbp_world_gm) ItemType SpawnTransform))

(fn `ShowPlayerName`
  (`/Engine/EditorBlueprintResources/StandardMacros.IsValid` (`self.NickName`)
    (:`Is Valid`
      (`TextRenderComponent.K2_SetText` (`self.NickName`) (`KismetTextLibrary.Conv_StringToText` (`self.PlayerName`))))))

(fn `ToolAction`
  (params (ToolEnum :type "/Game/Enums/E_Tool Enum" :default "NewEnumerator0"))
  (bind _returnvalue (`SkeletalMeshComponent.GetAnimInstance` (`self.Mesh`)))
  ;[1 1 1] Comment
  (if (`self.IsPlayAttack`)
    _
    (elif (`self.IsAxeEquip`)
      (`AnimInstance.Montage_Play` _returnvalue "/Game/Character/ABP/AM_Player.AM_Player" 1.0 "MontageLength" 0.05 true)
      (`AnimInstance.Montage_JumpToSection` _returnvalue (`KismetStringLibrary.Conv_StringToName` (`KismetStringLibrary.Concat_StrStr` (`|GetEnumeratorNameAsString` (`local.ToolEnum`)) "Attack")) "/Game/Character/ABP/AM_Player.AM_Player"))))

(fn `UnEquipToolItem`
  (params (Tool :type "Actor Object Reference"))
  (bind _tool (`local.Tool`))
  (bind _asabp_player (cast `/Game/Character/ABP/ABP_Player` (`SkeletalMeshComponent.GetAnimInstance` (`self.Mesh`))))
  (set `/Game/Character/ABP/ABP_Player.IsHoldingAxe` false _asabp_player)
  (`/Engine/EditorBlueprintResources/StandardMacros.IsValid` _tool
    (:`Is Valid`
      (`self.K2_DestroyActor` _tool)
      (return))
    (:`Is Not Valid`
      (`KismetSystemLibrary.PrintString` "Tool Actor 없음"))))

(fn `UpdateNickName`
  (params (Value :type "Text (by ref)"))
  (`TextRenderComponent.K2_SetText` (`self.NickName`) Value) ; 이름 업데이트하기
)

(fn `UserConstructionScript`
  (`parent.UserConstructionScript`))