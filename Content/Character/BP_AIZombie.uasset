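; Networked AI zombie character that melees players, takes axe damage and spawns trophy items.
; Attack montages are multicast and turn it toward the blackboard target on ending, while its attack collision damages players through their status component.
; Client-detected axe overlaps route through the owning player, with damage relayed via owner, server and multicast events.
; HP's RepNotify triggers death, updating animation and blackboard and stopping AI movement; loot spawns through the game mode's item manager.
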(event `MultiPlayMontage`
  ;[1 1 1] 공격 애니메이션
  (`self.PlayAttackMontage`)
  (add `AnimInstance.OnMontageEnded` (`SkeletalMeshComponent.GetAnimInstance` (`self.Mesh`)) (delegate `LoopPlayer`)))

(event `LoopPlayer`
  (params (Montage :type "AnimMontage Object Reference") (bInterrupted :type Boolean))
  ;[1 1 1] 공격 애니메이션
  (`self.LookPlayer`))

(event `Owner_DamagedByPlayer`
  (params (Atk :type "Float (double-precision)"))
  ;[1 1 1] 데미지 / 죽음
  (`self.Server_DamagedByPlayer` Atk))

(event `Owner_SpawnItem`
  ;[1 1 1] 전리품 생성
  (`self.Server_SpawnItem`))

(event `MultiStopMontage`
  ;[1 1 1] 공격 애니메이션
  (if (`AnimInstance.IsAnyMontagePlaying` (`SkeletalMeshComponent.GetAnimInstance` (`self.Mesh`)))
    (`AnimInstance.Montage_Stop` (`SkeletalMeshComponent.GetAnimInstance` (`self.Mesh`)) 0.2 (`self.AIZombieAnimMontage`))))

(event `Server_DamagedByPlayer`
  (params (Atk :type "Float (double-precision)"))
  ;[1 1 1] 데미지 / 죽음
  (`self.Multi_DamagedByPlayer` Atk))

(event `Server_SpawnItem`
  ;[1 1 1] 전리품 생성
  (`self.SpawnTrophyItem`))

(event `Multi_DamagedByPlayer`
  (params (Atk :type "Float (double-precision)"))
  ;[1 1 1] 데미지 / 죽음
  (`self.DamagedByPlayer` Atk))

(event `Multi_Dead`
  ;[1 1 1] 데미지 / 죽음
  (`self.Dead`))

(event `self.AttackCollision.OnComponentBeginOverlap`
  (params (OverlappedComponent :type "PrimitiveComponent Object Reference") (OtherActor :type "Actor Object Reference") (OtherComp :type "PrimitiveComponent Object Reference") (OtherBodyIndex :type Integer) (bFromSweep :type Boolean) (SweepResult :type "HitResult Structure (by ref)"))
  ;[1 1 1] Attacking
  (if (`KismetSystemLibrary.DoesImplementInterface` OtherActor "/Game/Character/BPI_PlayerIdentifier.BPI_PlayerIdentifier_C")
    (bind _asbp_player_character (cast `/Game/Character/BP_PlayerCharacter` OtherActor))
    (`KismetSystemLibrary.PrintString` "형변환 성공")
    (`/Game/BluePrints/Class/BP_PlayerStatus.Owner_GetDamaged` (`/Game/Character/BP_PlayerCharacter.BP_PlayerStatus` _asbp_player_character) (`self.AttackPoint`))))

(event `self.CapsuleComponent.OnComponentBeginOverlap`
  (params (OverlappedComponent :type "PrimitiveComponent Object Reference") (OtherActor :type "Actor Object Reference") (OtherComp :type "PrimitiveComponent Object Reference") (OtherBodyIndex :type Integer) (bFromSweep :type Boolean) (SweepResult :type "HitResult Structure (by ref)"))
  ;[1 1 1] Attacked By Player
  (`self.AttackedByPlayer` OtherActor))

(event `self.CapsuleComponent.OnComponentEndOverlap`
  (params (OverlappedComponent :type "PrimitiveComponent Object Reference") (OtherActor :type "Actor Object Reference") (OtherComp :type "PrimitiveComponent Object Reference") (OtherBodyIndex :type Integer))
  ;[1 1 1] Attacked By Player
  (cast `/Game/BluePrints/Object/Tool/BP_Axe` OtherActor) ; 도끼라면
  (if (`self.IsAttacked`)
    (set `self.IsAttacked` false)))

(fn `AttackedByPlayer`
  (params (actor :type "Actor Object Reference"))
  (`/Engine/EditorBlueprintResources/ActorMacros.Switch Has Authority`
    (:`Remote`
      (bind _asbp_axe (cast `/Game/BluePrints/Object/Tool/BP_Axe` (`local.actor`))
        (:`then`
          (bind _asbp_player_character (cast `/Game/Character/BP_PlayerCharacter` (`self.GetOwner` _asbp_axe)))
          (`/Game/Character/BP_PlayerCharacter.Owner_AttackZombie` _asbp_player_character self (`/Game/BluePrints/Object/Tool/BP_Axe.AxeAtk` _asbp_axe)))
        (:`CastFailed`
          (`KismetSystemLibrary.PrintString` "도끼가 아님"))))))

(fn `DamagedByPlayer`
  (params (Atk :type "Float (double-precision)"))
  (bind _output_get (set `self.ZombieHP` (- (`self.ZombieHP`) Atk)))
  (`KismetSystemLibrary.PrintString` (`KismetStringLibrary.Conv_DoubleToString` _output_get))
  (`KismetSystemLibrary.PrintString` (`KismetSystemLibrary.GetObjectName` self)))

(fn `Dead`
  (locals (IsDead :type Name :default "IsDead"))
  (bind _asabp_aizombie (cast `/Game/Character/ABP/ABP_AIZombie` (`SkeletalMeshComponent.GetAnimInstance` (`self.Mesh`)))) ; 애니메이션 죽은 상태로 처리
  (set `/Game/Character/ABP/ABP_AIZombie.IsDead` true _asabp_aizombie)
  (bind _asbp_aizombie_controller (cast `/Game/AI/AI_Zombie/BP_AIZombieController` (`AIBlueprintHelperLibrary.GetAIController` self)))
  (`Controller.StopMovement` _asbp_aizombie_controller) ; AI Controller 멈추기
  (`BlackboardComponent.SetValueAsBool` (`AIBlueprintHelperLibrary.GetBlackboard` _asbp_aizombie_controller) (`local.IsDead`) true) ; 죽은 상태로 전환
)

(fn `LookPlayer`
  (locals (Target :type Name :default "Target"))
  (bind _asbp_aizombie_controller (cast `/Game/AI/AI_Zombie/BP_AIZombieController` (`AIBlueprintHelperLibrary.GetAIController` null)))
  (bind _asbp_player_character (cast `/Game/Character/BP_PlayerCharacter` (`BlackboardComponent.GetValueAsObject` (`AIBlueprintHelperLibrary.GetBlackboard` _asbp_aizombie_controller) (`local.Target`))))
  (`self.K2_SetActorRotation` (`KismetMathLibrary.FindLookAtRotation` (`self.K2_GetActorLocation`) (`self.K2_GetActorLocation` _asbp_player_character))))

(fn `OnRep_ZombieHP`
  (if (<= (`self.ZombieHP`) 0.0)
    (`self.Multi_Dead`)))

(fn `PlayAttackMontage`
  (bind _returnvalue (`SkeletalMeshComponent.GetAnimInstance` (`self.Mesh`)))
  (if (not (`AnimInstance.IsAnyMontagePlaying` (`SkeletalMeshComponent.GetAnimInstance` (`self.Mesh`))))
    (`AnimInstance.Montage_Play` _returnvalue (`self.AIZombieAnimMontage`) 1.0 "MontageLength" 0.0 true)
    (`AnimInstance.Montage_JumpToSection` _returnvalue "Attack" (`self.AIZombieAnimMontage`))))

(fn `SpawnTrophyItem`
  (bind _asbp_world_gm (cast `/Game/BluePrints/GameMode/BP_WorldGM` (`GameplayStatics.GetGameMode`)))
  (`/Game/BluePrints/Class/BP_ItemManager.SpawnNewItem` (`/Game/BluePrints/GameMode/BP_WorldGM.BP_ItemManager` _asbp_world_gm) "NewEnumerator9" (`SceneComponent.K2_GetComponentToWorld` (`self.SpawnTransform`))))

(fn `UserConstructionScript`
  (`parent.UserConstructionScript`))